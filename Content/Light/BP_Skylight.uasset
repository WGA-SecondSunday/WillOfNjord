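; Skylight actor that drives a day/night cycle of light intensity and fog height from game time.
; On BeginPlay it spawns and configures a volumetric ExponentialHeightFog, and its construction script binds to the gamemode time manager's minute-change event.
; EarthRotate advances a wrapping angle counter, dimming and restoring the light within two angle windows.
; The fog height checks chain off those intensity steps, so fog lowers or rises only where the ranges meet.
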(event `self.ReceiveBeginPlay`
  (bind _returnvalue (`|SpawnActorFromClass` "/Script/Engine.ExponentialHeightFog" (`KismetMathLibrary.MakeTransform` (0.0 0.0 4700.0)) "AlwaysSpawn" "OverrideRootScale" null null))
  (bind _component (`ExponentialHeightFog.Component` _returnvalue))
  (`ExponentialHeightFogComponent.SetFogDensity` _component 0.02)
  (`ExponentialHeightFogComponent.SetFogHeightFalloff` _component 0.8)
  (`ExponentialHeightFogComponent.SetFogInscatteringColor` _component (make `LinearColor` 0.7 0.8 0.6 1.0))
  (`ActorComponent.SetAutoActivate` _component true)
  (`ExponentialHeightFogComponent.SetVolumetricFog` _component true)
  (`ExponentialHeightFogComponent.SetVolumetricFogDistance` (`ExponentialHeightFog.Component` _returnvalue) 10000.0))

(event `EarthRotate`
  (params (NewParam :type "/Game/BP_Core/TimeManagement/BP_GameTime Structure"))
  (bind _z_axis (`self.Z_Axis`))
  (bind _z_axis_2 (`self.Z_Axis`))
  (bind _z_axis_3 (`self.Z_Axis`))
  (bind _lightcomponent (`self.LightComponent`))
  (bind _z_axis_4 (`self.Z_Axis`))
  (bind _lightcomponent_2 (`self.LightComponent`))
  (bind _output_get (set `self.Z_Axis` (+ (`self.Z_Axis`) 2.5)))
  (if (>= _output_get 360.0)
    (set `self.Z_Axis` 0.0))
  (if (and (>= _z_axis_2 200.0) (<= _z_axis_2 215.0))
    (`SkyLightComponent.SetIntensity` _lightcomponent_2 (- (`LightComponentBase.Intensity` _lightcomponent_2) 0.5))
    (if (and (>= _z_axis_4 215.0) (<= _z_axis_4 230.0)) :!label _label
      (bind _returnvalue (`GameplayStatics.GetActorOfClass` "/Script/Engine.ExponentialHeightFog"))
      (bind _component (`ExponentialHeightFog.Component` _returnvalue))
      (`SceneComponent.K2_SetWorldLocation` _component (`KismetMathLibrary.MakeVector` 0.0 0.0 (- (.z (`SceneComponent.K2_GetComponentLocation` _component)) 30.0)) false false)
      (elif (and (>= _z_axis 345.0) (<= _z_axis 360.0))
        (bind _returnvalue_2 (`GameplayStatics.GetActorOfClass` "/Script/Engine.ExponentialHeightFog"))
        (bind _component_2 (`ExponentialHeightFog.Component` _returnvalue_2))
        (`SceneComponent.K2_SetWorldLocation` _component_2 (`KismetMathLibrary.MakeVector` 0.0 0.0 (+ (.z (`SceneComponent.K2_GetComponentLocation` _component_2)) 30.0)) false false)))
    (elif (and (>= _z_axis_3 330.0) (<= _z_axis_3 345.0))
      (`SkyLightComponent.SetIntensity` _lightcomponent (+ (`LightComponentBase.Intensity` _lightcomponent) 0.5))
      (goto _label))))

(fn `UserConstructionScript`
  (bind _asbp_gamemode (cast `/Game/BP_Core/BP_Gamemode` (`GameplayStatics.GetGameMode`)))
  (add `/Game/BP_Core/TimeManagement/BP_TimeManager.OnMinuteChange` (`/Game/BP_Core/BP_Gamemode.GTimeManager` _asbp_gamemode) (`|CreateDelegate` :!event `EarthRotate`)))