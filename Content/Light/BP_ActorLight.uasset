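; BP_ActorLight is a sun-light actor that animates a day cycle with two directional lights.
; The Construction Script binds to the game mode time manager's minute-change event and sets the main light's initial rotation and color.
; EarthRotate advances a wrapping angle by a fixed step, using sine and cosine to drive the main light's color and intensity alongside its rotation.
; The second light switches on only within a set angle range.
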(event `self.ReceiveBeginPlay`)

(event `self.ReceiveTick`
  (params (DeltaSeconds :type "Float (single-precision)")))

(event `EarthRotate`
  (params (NewParam :type "/Game/BP_Core/TimeManagement/BP_GameTime Structure"))
  (bind _z_axis (`self.Z_Axis`))
  (bind _output_get (set `self.Z_Axis` (+ (`self.Z_Axis`) 2.5)))
  (if (>= _output_get 360.0)
    (set `self.Z_Axis` 0.0))
  (`SceneComponent.K2_SetWorldRotation` (`self.DirectLight`) (`KismetMathLibrary.MakeRotator` 0.0 (`self.Z_Axis`) (+ (/ (- (`self.Z_Axis`) 180.0) 10.0) 70.0)) false false)
  (`LightComponent.SetLightColor` (`self.DirectLight`) (make `LinearColor` (+ (* (`KismetMathLibrary.DegSin` (`self.Z_Axis`)) 0.2) 0.8) (- (`self.Average_Green`) (* (`KismetMathLibrary.DegCos` (+ (`self.Z_Axis`) 180.0)) 0.3)) (- (`self.Average_Blue`) (* (`KismetMathLibrary.DegCos` (`self.Z_Axis`)) 0.2)) 1.0) true)
  (`LightComponent.SetIntensity` (`self.DirectLight`) (+ (* (`KismetMathLibrary.DegSin` (`self.Z_Axis`)) -2.0) 3.0))
  (if (or (>= _z_axis 150.0) (<= _z_axis 45.0))
    (`LightComponent.SetIntensity` (`self.DirectionalLight2`) 0.0)
    (else
      (`LightComponent.SetIntensity` (`self.DirectionalLight2`) 3.0))))

(fn `UserConstructionScript`
  (bind _asbp_gamemode (cast `/Game/BP_Core/BP_Gamemode` (`GameplayStatics.GetGameMode`)))
  (add `/Game/BP_Core/TimeManagement/BP_TimeManager.OnMinuteChange` (`/Game/BP_Core/BP_Gamemode.GTimeManager` _asbp_gamemode) (`|CreateDelegate` :!event `EarthRotate`))
  (`SceneComponent.K2_SetWorldRotation` (`self.DirectLight`) (`KismetMathLibrary.MakeRotator` 0.0 (`self.Z_Axis`) (+ (/ (- (`self.Z_Axis`) 180.0) 10.0) 70.0)) false false)
  (`LightComponent.SetLightColor` (`self.DirectLight`) (make `LinearColor` 0.8 (- (`self.Average_Green`) (* (`KismetMathLibrary.DegCos` (+ (`self.Z_Axis`) 180.0)) 0.3)) (- (`self.Average_Blue`) (* (`KismetMathLibrary.DegCos` (`self.Z_Axis`)) 0.2))) true))