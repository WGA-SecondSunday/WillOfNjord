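; Game event that runs a settlement's day cycle, setting the morning's conditions and resolving them at day end.
; Init rolls fog, rain or clear weather, sets the warrior quota and explorer cost per found person, then publishes the briefing.
; Deactivate removes weather efficiency modifiers by issuer, checks defense, food and wood, and downgrades or kills people by failure count.
; It then adds explorer-found people and building materials, and spawns a BP_GE_DayResults summary.
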(event `self.Init`
  (params (`Event Manager` :type "/Game/BP_Core/GameEventManagement/BP_GameEventManager Object Reference"))
  (`|ExecutionSequence`
    (:`then_1`
      (`parent.Init` `Event Manager`))
    (:`then_2`
      (`self.Create Conditions`))
    (:`then_3`
      (`self.Create Observer Requirement` `Event Manager`))
    (:`then_4`
      (`self.Make Self Description`))))

(fn `Activate`
  (params (Action :type Integer))
  (returns (Duration :type "/Game/BP_Core/TimeManagement/BP_GameTime Structure"))
  (bind _gtimemanager (`/Game/BP_Core/BP_Gamemode.GTimeManager` (`/Game/BP_Core/Base/BaseManager.GameManager` (`self.Event Manager`))))
  (`parent.Activate` 0)
  (return (`/Game/BP_Core/TimeManagement/BP_TimeFuncs.Game Time Delta` (`/Game/BP_Core/TimeManagement/BP_TimeManager.Work Day End Time` _gtimemanager) (`/Game/BP_Core/TimeManagement/BP_TimeManager.Work Day Start Time` _gtimemanager))))

(fn `Add Building Materials`
  (locals (Mat :type Integer))
  (bind _value (`BlueprintMapLibrary.Map_Find` (`/Game/BP_Core/ResourceManagement/BP_UResourceManager.Resources` (`/Game/BP_Core/BP_Gamemode.GResourceManager` (`/Game/BP_Core/Base/BaseManager.GameManager` (`self.Event Manager`)))) "NewEnumerator7"))
  (bind _output_get (set `local.Mat` (`self.Max Amount Of Materials`)))
  (`/Game/BP_Core/ResourceManagement/BP_UResource.UpdateAmount` _value (+ (`/Game/BP_Core/ResourceManagement/BP_UResource.Amount` _value) (`KismetMathLibrary.Conv_IntToDouble` _output_get))))

(fn `Cancel Weather Effect`
  (bind _gamemanager (`/Game/BP_Core/Base/BaseManager.GameManager` (`self.Event Manager`)))
  (for _array_element (`|MakeArray` "/Game/GameData/Professions/BP_Hunters.BP_Hunters_C" "/Game/GameData/Professions/BP_Woodcutters.BP_Woodcutters_C" "/Game/GameData/Professions/BP_Worker.BP_Worker_C" :!type "/Game/BP_Core/ProfessionManagement/BP_Profession Class Reference")
    (bind _global_efficiencies (`/Game/BP_Core/ProfessionManagement/BP_Profession.Global Efficiencies` (`BlueprintMapLibrary.Map_Find` (`/Game/BP_Core/ProfessionManagement/BP_ProfessionManager.Professions` (`/Game/BP_Core/BP_Gamemode.GProfessionsManager` (`/Game/BP_Core/Base/BaseManager.GameManager` (`self.Event Manager`)))) _array_element)))
    (bind (_arrayindex _arrayelement) (`/Engine/EditorBlueprintResources/StandardMacros.ReverseForEachLoop` _global_efficiencies)
      (:`LoopBody`
        (if (== self (break `/Game/BP_Core/ProfessionManagement/BP_EfficiencyModifier` _arrayelement))
          (`KismetArrayLibrary.Array_Remove` _global_efficiencies _arrayindex)))))
  (set `/Game/BP_Core/BP_Gamemode.Is Raining` false _gamemanager)
  (set `/Game/BP_Core/BP_Gamemode.Is Foggy` false _gamemanager))

(fn `Check Resource Conditions`
  (returns (`Is Food Satisfied` :type Boolean) (`Is Wood Satisfied` :type Boolean))
  (bind _resources (`/Game/BP_Core/ResourceManagement/BP_UResourceManager.Resources` (`/Game/BP_Core/BP_Gamemode.GResourceManager` (`/Game/BP_Core/Base/BaseManager.GameManager` (`self.Event Manager`)))))
  (return (> (`/Game/BP_Core/ResourceManagement/BP_UResource.Goal Reached Times` (`BlueprintMapLibrary.Map_Find` _resources "NewEnumerator0")) 0) (> (`/Game/BP_Core/ResourceManagement/BP_UResource.Goal Reached Times` (`BlueprintMapLibrary.Map_Find` _resources "NewEnumerator1")) 0)))

(fn `Check Warrior Condition`
  (returns (Satisfied :type Boolean))
  (bind _gamemanager (`/Game/BP_Core/Base/BaseManager.GameManager` (`self.Event Manager`)))
  (return (and (> (`/Game/BP_Core/ResourceManagement/BP_UResource.Goal Reached Times` (`BlueprintMapLibrary.Map_Find` (`/Game/BP_Core/ResourceManagement/BP_UResourceManager.Resources` (`/Game/BP_Core/BP_Gamemode.GResourceManager` _gamemanager)) "NewEnumerator10")) 0) (>= (`KismetArrayLibrary.Array_Length` (`/Game/BP_Core/ProfessionManagement/BP_Profession.Workers` (`BlueprintMapLibrary.Map_Find` (`/Game/BP_Core/ProfessionManagement/BP_ProfessionManager.Professions` (`/Game/BP_Core/BP_Gamemode.GProfessionsManager` _gamemanager)) "/Game/GameData/Professions/BP_Warriors.BP_Warriors_C"))) (`self.Warriors Required`)))))

(fn `Create And Apply Weather Effect`
  (locals (`Is Fog` :type Boolean) (`Is Rain` :type Boolean))
  (bind _gamemanager (`/Game/BP_Core/Base/BaseManager.GameManager` (`self.Event Manager`)))
  (bind _professions (`/Game/BP_Core/ProfessionManagement/BP_ProfessionManager.Professions` (`/Game/BP_Core/BP_Gamemode.GProfessionsManager` (`/Game/BP_Core/Base/BaseManager.GameManager` (`self.Event Manager`)))))
  (bind _output_get (set `local.Is Fog` (< (`KismetMathLibrary.RandomInteger` 100) (`self.Fog Probability`))))
  (if _output_get
    (set `/Game/BP_Core/BP_Gamemode.Is Foggy` true _gamemanager)
    (`KismetArrayLibrary.Array_Add` (`/Game/BP_Core/ProfessionManagement/BP_Profession.Global Efficiencies` (`BlueprintMapLibrary.Map_Find` _professions "/Game/GameData/Professions/BP_Hunters.BP_Hunters_C")) (make `/Game/BP_Core/ProfessionManagement/BP_EfficiencyModifier` self (`self.Fog Decreased Efficiency`)))
    (`KismetArrayLibrary.Array_Add` (`/Game/BP_Core/ProfessionManagement/BP_Profession.Global Efficiencies` (`BlueprintMapLibrary.Map_Find` _professions "/Game/GameData/Professions/BP_Woodcutters.BP_Woodcutters_C")) (make `/Game/BP_Core/ProfessionManagement/BP_EfficiencyModifier` self (`self.Fog Decreased Efficiency`)))
    (`KismetArrayLibrary.Array_Add` (`self.Day Begin Description Lines`) (`|FormatText` "- На улице туман. Производительность добычи еды и дерева снижена"))
    (else
      (bind _output_get_2 (set `local.Is Rain` (< (`KismetMathLibrary.RandomInteger` 100) (`self.Rain Probability`))))
      (if _output_get_2
        (set `/Game/BP_Core/BP_Gamemode.Is Raining` true _gamemanager)
        (`KismetArrayLibrary.Array_Add` (`/Game/BP_Core/ProfessionManagement/BP_Profession.Global Efficiencies` (`BlueprintMapLibrary.Map_Find` (`/Game/BP_Core/ProfessionManagement/BP_ProfessionManager.Professions` (`/Game/BP_Core/BP_Gamemode.GProfessionsManager` (`/Game/BP_Core/Base/BaseManager.GameManager` (`self.Event Manager`)))) "/Game/GameData/Professions/BP_Worker.BP_Worker_C")) (make `/Game/BP_Core/ProfessionManagement/BP_EfficiencyModifier` self (`self.Rain Decreased Efficiency`)))
        (`KismetArrayLibrary.Array_Add` (`self.Day Begin Description Lines`) (`|FormatText` "- На улице идет дождь. Скорость постройки зданий снижена"))
        (else
          (`KismetArrayLibrary.Array_Add` (`self.Day Begin Description Lines`) (`|FormatText` "- На улице ясная солнечная погода")))))))

(fn `Create Conditions`
  (bind _output_get (set `self.Warriors Required` (`KismetMathLibrary.FTrunc` (* (`KismetArrayLibrary.Array_Length` (`/Game/BP_Core/PeopleManagement/BP_PersonManager.People` (`/Game/BP_Core/BP_Gamemode.GPersonManager` (`/Game/BP_Core/Base/BaseManager.GameManager` (`self.Event Manager`))))) (`self.Warrior Percentage`)))))
  (`KismetArrayLibrary.Array_Add` (`self.Day Begin Description Lines`) (`|FormatText` "- Сегодня для защиты вашего поселения требуется назначить {num} воинов" _output_get))
  (`self.Create And Apply Weather Effect`))

(fn `Create Observer Requirement`
  (params (NewParam :type "/Game/BP_Core/GameEventManagement/BP_GameEventManager Object Reference"))
  (bind (_high _mid _low) (`/Game/BP_Core/PeopleManagement/BP_PersonManager.Get People Tags Count` (`/Game/BP_Core/BP_Gamemode.GPersonManager` (`/Game/BP_Core/Base/BaseManager.GameManager` NewParam))))
  (bind _output_get (set `self.People Found Requirement` (+ (* _high (`self.High Eff Found Coeff`)) (* _mid (`self.Mid Eff Found Coeff`)) (* _low (`self.Low Eff Found Coeff`)))))
  (`KismetSystemLibrary.PrintString` (`KismetTextLibrary.Conv_TextToString` (`|FormatText` "1 чел = {res} ресурса" _output_get)) true false (struct :`R` 0.046189 :`B` 1.0 :`A` 1.0))
  (return))

(fn `Deactivate`
  (locals (`Unsatisfied Conditions Count` :type Integer) (I :type Integer) (`Number Of People` :type Integer) (`People To Kill` :type "Array of Integer") (`Sorted Array` :type "Array of Object Object Reference"))
  (bind _unsatisfied_conditions_count (`local.Unsatisfied Conditions Count`))
  (bind _returnvalue (`KismetArrayLibrary.Array_Length` (`local.People To Kill`)))
  (bind _returnvalue_2 (- _unsatisfied_conditions_count 1))
  (bind _gamemanager (`/Game/BP_Core/Base/BaseManager.GameManager` (`self.Event Manager`)))
  (bind _returnvalue_3 (- (`local.Number Of People`) _returnvalue))
  (bind _ggameeventmanager (`/Game/BP_Core/BP_Gamemode.GGameEventManager` _gamemanager))
  (bind _gpersonmanager (`/Game/BP_Core/BP_Gamemode.GPersonManager` (`/Game/BP_Core/Base/BaseManager.GameManager` (`self.Event Manager`))))
  (bind _produced_events (`/Game/BP_Core/GameEventManagement/BP_GameEventManager.Produced Events` _ggameeventmanager))
  (bind _people (`/Game/BP_Core/PeopleManagement/BP_PersonManager.People` (`/Game/BP_Core/BP_Gamemode.GPersonManager` (`/Game/BP_Core/Base/BaseManager.GameManager` (`self.Event Manager`)))))
  (`parent.Deactivate`)
  (`self.Cancel Weather Effect`)
  (`|ExecutionSequence`
    (:`then_0`
      (bind _satisfied (`self.Check Warrior Condition`))
      (if _satisfied
        (`KismetArrayLibrary.Array_Add` (`self.Day End Description Lines`) (`|FormatText` "- Ваши воины успешно защитили поселение от диких зверей и варваров! \n"))
        (else
          (`/Engine/EditorBlueprintResources/StandardMacros.IncrementInt` (`local.Unsatisfied Conditions Count`)
            (:`  `
              (`KismetArrayLibrary.Array_Add` (`self.Day End Description Lines`) (`|FormatText` "- Ваши воины не смогли обеспечить достаточную защиту! \n")))))))
    (:`then_1`
      (bind (_is_food_satisfied _is_wood_satisfied) (`self.Check Resource Conditions`))
      (`|ExecutionSequence`
        (:`then_0`
          (if _is_food_satisfied
            (`KismetArrayLibrary.Array_Add` (`self.Day End Description Lines`) (`|FormatText` "- Вы полностью удовлетворили потребности населения в еде \n"))
            (else
              (`/Engine/EditorBlueprintResources/StandardMacros.IncrementInt` (`local.Unsatisfied Conditions Count`)
                (:`  `
                  (`KismetArrayLibrary.Array_Add` (`self.Day End Description Lines`) (`|FormatText` "- Вашим жителям не хватило еды! \n")))))))
        (:`then_1`
          (if _is_wood_satisfied
            (`KismetArrayLibrary.Array_Add` (`self.Day End Description Lines`) (`|FormatText` "- Вы полностью удовлетворили потребности населения в дереве  \n"))
            (else
              (`/Engine/EditorBlueprintResources/StandardMacros.IncrementInt` (`local.Unsatisfied Conditions Count`)
                (:`  `
                  (`KismetArrayLibrary.Array_Add` (`self.Day End Description Lines`) (`|FormatText` "- Вашим жителям не хватило еды! \n")))))))))
    (:`then_2`
      (if (>= _unsatisfied_conditions_count 0)
        (set `local.Number Of People` (+ (`|GetArrayItem` (`self.Constant People Remove Counts`) _returnvalue_2) (`KismetMathLibrary.FTrunc` (* (`KismetArrayLibrary.Array_Length` (`/Game/BP_Core/PeopleManagement/BP_PersonManager.People` _gpersonmanager)) (`|GetArrayItem` (`self.People Remove Percentages`) _returnvalue_2)))))
        (bind _sorted (`/Game/BP_Core/PeopleManagement/BP_PersonManager.Get Sorted People` _gpersonmanager))
        (set `local.Sorted Array` _sorted)
        (while (< (`local.I`) (`local.Number Of People`))
          (bind _asbp_person (cast `/Game/BP_Core/PeopleManagement/BP_Person` (`|GetArrayItem` (`local.Sorted Array`) (`local.I`))))
          (bind _tag (`/Game/BP_Core/PeopleManagement/BP_Person.Get Efficiency Tag` _asbp_person))
          (bind _must_be_killed (`/Game/BP_Core/PeopleManagement/BP_PersonManager.Set People Eff Tag` _gpersonmanager _asbp_person (+ _tag 1)))
          (if _must_be_killed
            (`KismetArrayLibrary.Array_Add` (`local.People To Kill`) (`local.I`)))
          (`/Engine/EditorBlueprintResources/StandardMacros.IncrementInt` (`local.I`)))))
    (:`then_3`
      (if (> _returnvalue_3 0)
        (`KismetArrayLibrary.Array_Add` (`self.Day End Description Lines`) (`|FormatText` "- В результате невыполнения условий {num} человек стали менее эффективными! \n" _returnvalue_3)))
      (if (> _returnvalue 0)
        (`KismetArrayLibrary.Array_Add` (`self.Day End Description Lines`) (`|FormatText` "- В результате невыполнения условий {num} человек погибли! \n" _returnvalue))
        (bind (_arrayindex _arrayelement) (`/Engine/EditorBlueprintResources/StandardMacros.ReverseForEachLoop` (`local.People To Kill`))
          (:`LoopBody`
            (bind _output (`|GetArrayItem` _people _arrayelement))
            (`/Game/BP_Core/PeopleManagement/BP_Person.FireFromWork` _output)
            (`Actor.K2_DestroyActor` (`/Game/BP_Core/PeopleManagement/BP_Person.Linked AI` _output))
            (`KismetArrayLibrary.Array_Remove` _people _arrayelement)))))
    (:`then_4`
      (`self.Make Observer Effect`)
      (`self.Add Building Materials`))
    (:`then_5`
      (bind _returnvalue_4 (`|GenericCreateObject` "/Game/GameData/GameEvents/DayBeginEndEvents/BP_GE_DayResults.BP_GE_DayResults_C" self "Итоги дня"))
      (`/Game/GameData/GameEvents/DayBeginEndEvents/BP_GE_DayResults.Make Description` _returnvalue_4 (`self.Day End Description Lines`))
      (`KismetArrayLibrary.Array_Clear` _produced_events)
      (`KismetArrayLibrary.Array_Add` _produced_events _returnvalue_4)
      (`/Game/BP_Core/GameEventManagement/BP_GameEventManager.Produced Event Handler` _ggameeventmanager null)
      (`Widget.SetIsEnabled` (`/Game/UI/Widgets/TimerAndScreenButtons/BP_HUD.EventButton` (`/Game/BP_Core/BP_Gamemode.WHUD` _gamemanager)) false))))

(fn `Make Observer Effect`
  (locals (Chance :type Integer) (`Number Of People` :type Integer))
  (bind _gamemanager (`/Game/BP_Core/Base/BaseManager.GameManager` (`self.Event Manager`)))
  (bind _gpersonmanager (`/Game/BP_Core/BP_Gamemode.GPersonManager` _gamemanager))
  (bind _returnvalue (- (`/Game/BP_Core/PeopleManagement/BP_PersonManager.MaxPeople` _gpersonmanager) (`KismetArrayLibrary.Array_Length` (`/Game/BP_Core/PeopleManagement/BP_PersonManager.People` _gpersonmanager))))
  (bind _returnvalue_2 (`KismetMathLibrary.FTrunc` (/ (`/Game/BP_Core/ResourceManagement/BP_UResource.Amount` (`BlueprintMapLibrary.Map_Find` (`/Game/BP_Core/ResourceManagement/BP_UResourceManager.Resources` (`/Game/BP_Core/BP_Gamemode.GResourceManager` _gamemanager)) "NewEnumerator9")) (`self.People Found Requirement`))))
  (if (> _returnvalue_2 0)
    (bind _output_get (set `local.Number Of People` _returnvalue_2))
    (if (> _output_get _returnvalue)
      (set `local.Number Of People` _returnvalue))
    (`/Game/BP_Core/PeopleManagement/BP_PersonManager.Add People` _gpersonmanager _output_get true)
    (`KismetArrayLibrary.Array_Add` (`self.Day End Description Lines`) (`|FormatText` "- Исследователи нашли {number} людей! \n" _output_get))
    (else
      (`KismetArrayLibrary.Array_Add` (`self.Day End Description Lines`) (`|FormatText` "- Исследователи не смогли ничего найти за день \n")))))

(fn `Make Self Description`
  (locals (`Final Text` :type String))
  (bind _event_manager (`self.Event Manager`))
  (bind (_title _content _actionsandconsequences) (break `/Game/BP_Core/GameEventManagement/BP_GameEventTexts` (`self.Texts`)))
  (for _array_element (`self.Day Begin Description Lines`)
    (set `local.Final Text` (`KismetStringLibrary.Concat_StrStr` (`local.Final Text`) (`KismetTextLibrary.Conv_TextToString` _array_element) " \n")))
  (bind _output_get (set `self.Texts` (make `/Game/BP_Core/GameEventManagement/BP_GameEventTexts` _title (`KismetTextLibrary.Conv_StringToText` (`local.Final Text`)) _actionsandconsequences)))
  (set `/Game/BP_Core/GameEventManagement/BP_GameEventManager.Current Day Conditions` _output_get _event_manager)
  (`Widget.SetIsEnabled` (`/Game/UI/Widgets/TimerAndScreenButtons/BP_HUD.EventButton` (`/Game/BP_Core/BP_Gamemode.WHUD` (`/Game/BP_Core/Base/BaseManager.GameManager` _event_manager))) true))

(fn `Random Death Or Efficiency Decrease`
  (params (Reason :type Text))
  (locals (I :type Integer) (`Number Of People` :type Integer))
  (bind _people (`/Game/BP_Core/PeopleManagement/BP_PersonManager.People` (`/Game/BP_Core/BP_Gamemode.GPersonManager` (`/Game/BP_Core/Base/BaseManager.GameManager` (`self.Event Manager`)))))
  (bind (_outitem _outindex) (`KismetArrayLibrary.Array_Random` _people))
  (bind _outitem_2 (`KismetArrayLibrary.Array_Random` (`/Game/BP_Core/PeopleManagement/BP_PersonManager.People` (`/Game/BP_Core/BP_Gamemode.GPersonManager` (`/Game/BP_Core/Base/BaseManager.GameManager` (`self.Event Manager`))))))
  (set `local.Number Of People` (`KismetMathLibrary.RandomIntegerInRange` 1 (`self.Maximum Affected By Negative Effect`)))
  (if (< (`KismetMathLibrary.RandomIntegerInRange` 0 100) (`self.Death Probability`))
    (while (< (`local.I`) (`local.Number Of People`))
      (`/Engine/EditorBlueprintResources/StandardMacros.IncrementInt` (`local.I`)
        (:`  `
          (`/Game/BP_Core/PeopleManagement/BP_Person.FireFromWork` _outitem)
          (`KismetArrayLibrary.Array_Remove` _people _outindex))))
    (`KismetArrayLibrary.Array_Add` (`self.Day End Description Lines`) (`|FormatText` "- Вы потеряли {num} своего (-их) жителя (-ей) из-за {reason} \n" (`local.Number Of People`) Reason))
    (else
      (while (< (`local.I`) (`local.Number Of People`))
        (`/Engine/EditorBlueprintResources/StandardMacros.IncrementInt` (`local.I`)
          (:`  `
            (set `/Game/BP_Core/PeopleManagement/BP_Person.Efficiency` (`KismetMathLibrary.RandomFloatInRange` (`self.Minimum Decreased Efficiency`) (`/Game/BP_Core/PeopleManagement/BP_Person.Efficiency` _outitem_2)) _outitem_2))))
      (`KismetArrayLibrary.Array_Add` (`self.Day End Description Lines`) (`|FormatText` "- {num} житель (-я) заболело и ослабло из-за {reason} \n" (`local.Number Of People`) Reason)))))