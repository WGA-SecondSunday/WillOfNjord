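; Game event Blueprint for the day results screen, shown among the day begin and end events.
; Its Make Description function loops over an array of texts and appends each into one string.
; The combined string becomes the content of a game event texts struct, keeping the title and passing the incoming actions through.
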(fn `Make Description`
  (params (Texts :type "Array of Text"))
  (locals (`Final Text` :type String))
  (for _array_element Texts
    (set `local.Final Text` (`KismetStringLibrary.Concat_StrStr` (`local.Final Text`) (`KismetTextLibrary.Conv_TextToString` _array_element))))
  (set `self.Texts` (make `/Game/BP_Core/GameEventManagement/BP_GameEventTexts` (`self.Title`) (`KismetTextLibrary.Conv_StringToText` (`local.Final Text`)) (`.Actions_10_DDD891E2410792AFB01766A1CCD7D206` (break `/Game/BP_Core/GameEventManagement/BP_GameEventTexts` (`self.Texts`))))))