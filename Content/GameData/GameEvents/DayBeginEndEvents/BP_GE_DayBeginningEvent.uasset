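; Game event for the beginning of a day, which schedules that day's end action and announces its warrior requirement.
; On Init it wraps a new day-end action in a deferred action, timed by the difference between the day-end and day-begin event times in the event manager's static data.
; After parent initialization, it inserts the action's required warrior count into the event's content text.
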(event `self.Init`
  (params (`Event Manager` :type "/Game/BP_Core/GameEventManagement/BP_GameEventManager Object Reference"))
  (bind _static_data (`/Game/BP_Core/GameEventManagement/BP_GameEventManager.Static Data` `Event Manager`))
  (bind (_texts_title _texts_content _texts_actions) (break `/Game/BP_Core/GameEventManagement/BP_GameEventTexts` (`self.Texts`)))
  (`|ExecutionSequence`
    (:`then_1`
      (`|ExecutionSequence`
        (:`then_0`
          (bind _returnvalue (`|GenericCreateObject` "/Game/GameData/GameEvents/DayBeginEndEvents/Actions/BP_DayEndAction.BP_DayEndAction_C" self))
          (bind _returnvalue_2 (`|GenericCreateObject` "/Game/GameData/GameEvents/Actions/BP_GEA_DefferedAction.BP_GEA_DefferedAction_C" self _returnvalue))
          (`KismetArrayLibrary.Array_Add` (`self.Actions`) (make `/Game/BP_Core/GameEventManagement/S_ActionAndDuration` _returnvalue_2 (`/Game/BP_Core/TimeManagement/BP_TimeFuncs.Game Time Delta` (`/Game/BP_Core/GameEventManagement/BPDA_GameEvents.Day End Event Time` _static_data) (`/Game/BP_Core/GameEventManagement/BPDA_GameEvents.Day Begin Event Time` _static_data)))))))
    (:`then_2`
      (`parent.Init` `Event Manager`))
    (:`then_3`
      (set `self.Texts` (make `/Game/BP_Core/GameEventManagement/BP_GameEventTexts` _texts_title (`|FormatText` _texts_content (`/Game/GameData/GameEvents/DayBeginEndEvents/Actions/BP_DayEndAction.Required Warriors` _returnvalue)) _texts_actions)))))

(fn `Create Texts`
  (locals (Content :type Text :default "NSLOCTEXT(\"\", \"8555E54E435CBC1C5C255983014EFAC6\", \"Сегодня требуется {} воинов. \")"))
  (bind (_title _content _actions) (break `/Game/BP_Core/GameEventManagement/BP_GameEventTexts` (`self.Texts`)))
  (set `self.Texts` (make `/Game/BP_Core/GameEventManagement/BP_GameEventTexts` _title _content _actions)))