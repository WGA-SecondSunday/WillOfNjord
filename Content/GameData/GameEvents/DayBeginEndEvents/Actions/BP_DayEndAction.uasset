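; BP_DayEndAction is a game event action that decides whether the day ends well or badly based on how many warriors the population has.
; Init caches the game mode and sets the warrior requirement to a quarter of the current population.
; Enable compares the Warriors profession's worker count to that requirement and constructs a good or bad day-ending event.
; It queues that event in the game event manager and triggers its handler.
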(event `self.Init`
  (params (Holder :type "/Game/BP_Core/GameEventManagement/BP_GameEvent Object Reference"))
  (`parent.Init` Holder)
  (bind _output_get (set `self.Gamemode` (`/Game/BP_Core/Base/BaseManager.GameManager` (`/Game/BP_Core/GameEventManagement/BP_GameEvent.Event Manager` Holder))))
  (set `self.Required Warriors` (/ (`KismetArrayLibrary.Array_Length` (`/Game/BP_Core/PeopleManagement/BP_PersonManager.People` (`/Game/BP_Core/BP_Gamemode.GPersonManager` _output_get))) 4)))

(fn `Check Conditions`
  (returns (Satisfied :type Boolean))
  (return (>= (`KismetArrayLibrary.Array_Length` (`/Game/BP_Core/ProfessionManagement/BP_Profession.Workers` (`BlueprintMapLibrary.Map_Find` (`/Game/BP_Core/ProfessionManagement/BP_ProfessionManager.Professions` (`/Game/BP_Core/BP_Gamemode.GProfessionsManager` (`self.Gamemode`))) "/Game/GameData/Professions/BP_Warriors.BP_Warriors_C"))) (`self.Required Warriors`))))

(fn `Enable`
  (locals (`Generated Event` :type "/Game/BP_Core/GameEventManagement/BP_GameEvent Object Reference"))
  (bind _generated_event (`local.Generated Event`))
  (bind _ggameeventmanager (`/Game/BP_Core/BP_Gamemode.GGameEventManager` (`self.Gamemode`)))
  (`parent.Enable`)
  (bind _satisfied (`self.Check Conditions`))
  (if _satisfied
    (bind _returnvalue (`|GenericCreateObject` "/Game/GameData/GameEvents/DayBeginEndEvents/BP_GE_GoodDayEnding.BP_GE_GoodDayEnding_C" self))
    (set `local.Generated Event` _returnvalue)
    (else
      (bind _returnvalue_2 (`|GenericCreateObject` "/Game/GameData/GameEvents/DayBeginEndEvents/BP_GE_BadDayEnding.BP_GE_BadDayEnding_C" self))
      (set `local.Generated Event` _returnvalue_2)))
  (`/Game/BP_Core/GameEventManagement/BP_GameEvent.Init` _generated_event null)
  (`KismetArrayLibrary.Array_Add` (`/Game/BP_Core/GameEventManagement/BP_GameEventManager.Produced Events` _ggameeventmanager) _generated_event)
  (`/Game/BP_Core/GameEventManagement/BP_GameEventManager.Produced Event Handler` _ggameeventmanager null))