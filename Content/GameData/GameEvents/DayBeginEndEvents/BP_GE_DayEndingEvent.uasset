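; BP_GE_DayEndingEvent is a game event Blueprint, named and filed as a day-ending event.
; Its Init event has an empty body, while a disconnected sequence would add a BP_GEA_DoNothing action and then call the parent Init.
; CreateTexts rebuilds the Texts struct from its existing title, content and action texts.
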(event `self.Init`
  (params (`Event Manager` :type "/Game/BP_Core/GameEventManagement/BP_GameEventManager Object Reference")))

(fn `Create Texts`
  (locals (Content :type Text :default "NSLOCTEXT(\"\", \"8555E54E435CBC1C5C255983014EFAC6\", \"Сегодня требуется {} воинов. \")"))
  (bind (_title _content _actions) (break `/Game/BP_Core/GameEventManagement/BP_GameEventTexts` (`self.Texts`)))
  (set `self.Texts` (make `/Game/BP_Core/GameEventManagement/BP_GameEventTexts` _title _content _actions)))