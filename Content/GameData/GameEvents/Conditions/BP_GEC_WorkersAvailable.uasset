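; A game event condition that passes when enough workers exist in a given profession.
; CheckSelf reaches the professions manager through the holder event's event manager and game manager, looks up the configured Profession, and compares its worker count to NumberOfWorkers.
; The check counts all workers listed under that profession and uses a greater-or-equal threshold.
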(fn `CheckSelf`
  (returns (Result :type Boolean))
  (return (>= (`KismetArrayLibrary.Array_Length` (`/Game/BP_Core/ProfessionManagement/BP_Profession.Workers` (`BlueprintMapLibrary.Map_Find` (`/Game/BP_Core/ProfessionManagement/BP_ProfessionManager.Professions` (`/Game/BP_Core/BP_Gamemode.GProfessionsManager` (`/Game/BP_Core/Base/BaseManager.GameManager` (`/Game/BP_Core/GameEventManagement/BP_GameEvent.Event Manager` (`self.Holder Event`))))) (`self.Profession`)))) (`self.Number of Workers`))))