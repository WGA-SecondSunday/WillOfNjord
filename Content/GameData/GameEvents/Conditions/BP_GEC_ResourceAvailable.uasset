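; BP_GEC_ResourceAvailable is a game event condition that passes when the game holds at least a required amount of a given resource.
; CheckSelf looks up the Resource in the resource manager's map, reached through the holder event's event manager and game manager.
; It returns true only when that entry exists and its amount meets or exceeds the configured Amount, otherwise false.
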(fn `CheckSelf`
  (returns (Result :type Boolean))
  (bind (_value _returnvalue) (`BlueprintMapLibrary.Map_Find` (`/Game/BP_Core/ResourceManagement/BP_UResourceManager.Resources` (`/Game/BP_Core/BP_Gamemode.GResourceManager` (`/Game/BP_Core/Base/BaseManager.GameManager` (`/Game/BP_Core/GameEventManagement/BP_GameEvent.Event Manager` (`self.Holder Event`))))) (`self.Resource`)))
  (if _returnvalue
    (if (>= (`/Game/BP_Core/ResourceManagement/BP_UResource.Amount` _value) (`self.Amount`))
      (return true)
      (else
        (return false)))
    (else
      (return false))))