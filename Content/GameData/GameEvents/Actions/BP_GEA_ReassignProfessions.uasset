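; BP_GEA_ReassignProfessions is a game event action that moves a set number of workers from one profession to another.
; On Enable it calls the parent, then loops Amount times over data from the professions manager, reached through the holder event.
; Each pass fires the last worker of FromProfession and assigns them to ToProfession, bypassing its maximum worker limit.
; It does not check whether the source profession has enough workers.
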(fn `Enable`
  (locals (I :type Integer) (People :type "/Game/BP_Core/PeopleManagement/BP_Person Object Reference"))
  (bind _professions (`/Game/BP_Core/ProfessionManagement/BP_ProfessionManager.Professions` (`/Game/BP_Core/BP_Gamemode.GProfessionsManager` (`/Game/BP_Core/Base/BaseManager.GameManager` (`/Game/BP_Core/GameEventManagement/BP_GameEvent.Event Manager` (`self.Holder Event`))))))
  (bind _workers (`/Game/BP_Core/ProfessionManagement/BP_Profession.Workers` (`BlueprintMapLibrary.Map_Find` _professions (`self.From Profession`))))
  (`parent.Enable`)
  (while (< (`local.I`) (`self.Amount`))
    (`/Engine/EditorBlueprintResources/StandardMacros.IncrementInt` (`local.I`)
      (:`  `
        (bind _output_get (set `local.People` (`|GetArrayItem` _workers (- (`KismetArrayLibrary.Array_Length` _workers) 1))))
        (`/Game/BP_Core/PeopleManagement/BP_Person.FireFromWork` _output_get)
        (`/Game/BP_Core/ProfessionManagement/BP_Profession.AssignWorker` (`BlueprintMapLibrary.Map_Find` _professions (`self.To Profession`)) _output_get true)))))