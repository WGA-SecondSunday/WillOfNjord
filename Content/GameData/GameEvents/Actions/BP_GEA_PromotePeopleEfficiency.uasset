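; Game event action that raises the efficiency of the least efficient people in the game's person manager.
; On Enable it calls the parent, then loops for a configurable fraction of the population count, truncated to a whole number.
; Each pass rescans the full list for the lowest efficiency below MinimumEfficiency and multiplies that person's value by EfficiencyIncreaseFactor, so one person can be boosted repeatedly.
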(fn `Enable`
  (locals (I :type Integer))
  (bind _people (`/Game/BP_Core/PeopleManagement/BP_PersonManager.People` (`/Game/BP_Core/BP_Gamemode.GPersonManager` (`/Game/BP_Core/Base/BaseManager.GameManager` (`/Game/BP_Core/GameEventManagement/BP_GameEvent.Event Manager` (`self.Holder Event`))))))
  (`parent.Enable`)
  (while (< (`local.I`) (`KismetMathLibrary.FTrunc` (* (`KismetArrayLibrary.Array_Length` _people) (`self.Promotion Amount Percentage`))))
    (`/Engine/EditorBlueprintResources/StandardMacros.IncrementInt` (`local.I`)
      (:`  `
        (bind _ret (`self.Get Minimum Effective Person` _people))
        (set `/Game/BP_Core/PeopleManagement/BP_Person.Efficiency` (* (`/Game/BP_Core/PeopleManagement/BP_Person.Efficiency` _ret) (`self.Efficiency Increase Factor`)) _ret)))))

(fn `Get Minimum Effective Person`
  (params (NewParam :type "Array of /Game/BP_Core/PeopleManagement/BP_Person Object Reference"))
  (returns (Ret :type "/Game/BP_Core/PeopleManagement/BP_Person Object Reference"))
  (locals (`Minimum Efficiency` :type "Float (double-precision)" :default 3.4028234663852886e+38) (Person :type "/Game/BP_Core/PeopleManagement/BP_Person Object Reference"))
  (for _array_element NewParam
    (if (< (`/Game/BP_Core/PeopleManagement/BP_Person.Efficiency` _array_element) (`local.Minimum Efficiency`))
      (set `local.Minimum Efficiency` (`/Game/BP_Core/PeopleManagement/BP_Person.Efficiency` _array_element))
      (set `local.Person` _array_element)))
  (return (`local.Person`)))