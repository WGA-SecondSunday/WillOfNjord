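; BP_GEA_DefferedAction is a game event action that wraps another Action and defers it until the wrapper is disabled.
; Init and Deinit call the parent, then forward to the wrapped Action, passing the Holder on Init.
; Enable only runs parent logic, while Disable calls the parent, then immediately enables and disables the wrapped Action, firing it as a one-shot pulse at the end.
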(event `self.Init`
  (params (Holder :type "/Game/BP_Core/GameEventManagement/BP_GameEvent Object Reference"))
  (`parent.Init` Holder)
  (`self.Init` (`self.Action`) Holder))

(event `self.Deinit`
  (`parent.Deinit`)
  (`self.Deinit` (`self.Action`)))

(fn `Disable`
  (bind _action (`self.Action`))
  (`parent.Disable`)
  (`self.Enable` _action)
  (`self.Disable` _action))

(fn `Enable`
  (`parent.Enable`))