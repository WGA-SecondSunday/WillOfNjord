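; Game event action that sends a set Amount of random people to the rest profession for RestDuration when enabled.
; It loops over random picks from the person manager, skips indices in AlreadyResting, and assigns workers through BP_RestProfession.
; The pure Random node re-evaluates per step, so checked, assigned and recorded people can differ.
; The loop has no exit if Amount exceeds the available people.
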(fn `Enable`
  (locals (`Already Resting` :type "Array of Integer") (I :type Integer))
  (bind _gamemanager (`/Game/BP_Core/Base/BaseManager.GameManager` (`/Game/BP_Core/GameEventManagement/BP_GameEvent.Event Manager` (`self.Holder Event`))))
  (bind (_outitem _outindex) (`KismetArrayLibrary.Array_Random` (`/Game/BP_Core/PeopleManagement/BP_PersonManager.People` (`/Game/BP_Core/BP_Gamemode.GPersonManager` _gamemanager))))
  (`parent.Enable`)
  (while (< (`local.I`) (`self.Amount`))
    (if (not (`KismetArrayLibrary.Array_Contains` (`local.Already Resting`) _outindex))
      (`/Game/GameData/Professions/BP_RestProfession.Assign Worker` (cast `/Game/GameData/Professions/BP_RestProfession` (`BlueprintMapLibrary.Map_Find` (`/Game/BP_Core/ProfessionManagement/BP_ProfessionManager.Professions` (`/Game/BP_Core/BP_Gamemode.GProfessionsManager` _gamemanager)) "/Game/GameData/Professions/BP_RestProfession.BP_RestProfession_C") :!pure true) _outitem (`self.Rest Duration`))
      (`/Engine/EditorBlueprintResources/StandardMacros.IncrementInt` (`local.I`)
        (:`  `
          (`KismetArrayLibrary.Array_Add` (`local.Already Resting`) _outindex))))))