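; Game event action that temporarily applies an efficiency modifier to one profession while it is enabled.
; Enable appends the efficiency, tagged with the action as issuer, to that profession's GlobalEfficiencies in the professions manager, reached through the holder event.
; Disable walks the list in reverse and removes every entry this action issued, leaving other modifiers intact.
; Both print Russian debug messages.
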(fn `Disable`
  (bind _global_efficiencies (`/Game/BP_Core/ProfessionManagement/BP_Profession.Global Efficiencies` (`BlueprintMapLibrary.Map_Find` (`/Game/BP_Core/ProfessionManagement/BP_ProfessionManager.Professions` (`/Game/BP_Core/BP_Gamemode.GProfessionsManager` (`/Game/BP_Core/Base/BaseManager.GameManager` (`/Game/BP_Core/GameEventManagement/BP_GameEvent.Event Manager` (`self.Holder Event`))))) (`self.Profession`))))
  (`parent.Disable`)
  (bind (_arrayindex _arrayelement) (`/Engine/EditorBlueprintResources/StandardMacros.ReverseForEachLoop` _global_efficiencies)
    (:`LoopBody`
      (if (== (break `/Game/BP_Core/ProfessionManagement/BP_EfficiencyModifier` _arrayelement) self)
        (`KismetArrayLibrary.Array_Remove` _global_efficiencies _arrayindex)))
    (:`Completed`
      (`KismetSystemLibrary.PrintString` null "Эффективность восстановлена"))))

(fn `Enable`
  (`parent.Enable`)
  (`KismetArrayLibrary.Array_Add` (`/Game/BP_Core/ProfessionManagement/BP_Profession.Global Efficiencies` (`BlueprintMapLibrary.Map_Find` (`/Game/BP_Core/ProfessionManagement/BP_ProfessionManager.Professions` (`/Game/BP_Core/BP_Gamemode.GProfessionsManager` (`/Game/BP_Core/Base/BaseManager.GameManager` (`/Game/BP_Core/GameEventManagement/BP_GameEvent.Event Manager` (`self.Holder Event`))))) (`self.Profession`))) (make `/Game/BP_Core/ProfessionManagement/BP_EfficiencyModifier` self (`self.Applied Efficiency`)))
  (`KismetSystemLibrary.PrintString` null "Новая эффективность установлена"))