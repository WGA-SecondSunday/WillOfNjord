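; Game event action that pulls a set number of workers from a chosen profession and sends them to rest for a given duration.
; When enabled, it looks up the profession through the event's game manager and acts only if that profession has enough workers.
; It repeatedly takes the first worker in the list, fires them and assigns them to the rest profession.
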(fn `Enable`
  (locals (Person :type "/Game/BP_Core/PeopleManagement/BP_Person Object Reference"))
  (bind _professions (`/Game/BP_Core/ProfessionManagement/BP_ProfessionManager.Professions` (`/Game/BP_Core/BP_Gamemode.GProfessionsManager` (`/Game/BP_Core/Base/BaseManager.GameManager` (`/Game/BP_Core/GameEventManagement/BP_GameEvent.Event Manager` (`self.Holder Event`))))))
  (bind _workers (`/Game/BP_Core/ProfessionManagement/BP_Profession.Workers` (`BlueprintMapLibrary.Map_Find` _professions (`self.Profession`))))
  (`parent.Enable`)
  (if (>= (`KismetArrayLibrary.Array_Length` _workers) (`self.Number of People`))
    (for _ (range (`self.Number of People`))
      (bind _output_get (set `local.Person` (`|GetArrayItem` _workers)))
      (`/Game/BP_Core/PeopleManagement/BP_Person.FireFromWork` _output_get)
      (`/Game/GameData/Professions/BP_RestProfession.Assign Worker` (cast `/Game/GameData/Professions/BP_RestProfession` (`BlueprintMapLibrary.Map_Find` _professions "/Game/GameData/Professions/BP_RestProfession.BP_RestProfession_C") :!pure true) _output_get (`self.Rest Duration`)))))