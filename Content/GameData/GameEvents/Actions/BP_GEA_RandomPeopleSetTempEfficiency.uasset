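; Game event action that temporarily scales a random resident's Efficiency by EfficiencyFactor while enabled.
; Enable draws from the GPersonManager People list, reached through the holder event, to store OldEfficiency and People and apply the multiplier.
; Random is evaluated separately for each access, so the saved value, stored resident and modified resident can differ.
; Disable writes OldEfficiency back to the stored resident; both functions print debug messages.
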(fn `Disable`
  (`parent.Disable`)
  (set `/Game/BP_Core/PeopleManagement/BP_Person.Efficiency` (`self.Old Efficiency`) (`self.People`))
  (`KismetSystemLibrary.PrintString` null "Снята временная эффективность с  жителю"))

(fn `Enable`
  (bind _outitem (`KismetArrayLibrary.Array_Random` (`/Game/BP_Core/PeopleManagement/BP_PersonManager.People` (`/Game/BP_Core/BP_Gamemode.GPersonManager` (`/Game/BP_Core/Base/BaseManager.GameManager` (`/Game/BP_Core/GameEventManagement/BP_GameEvent.Event Manager` (`self.Holder Event`)))))))
  (bind _efficiency (`/Game/BP_Core/PeopleManagement/BP_Person.Efficiency` _outitem))
  (`parent.Enable`)
  (set `self.Old Efficiency` _efficiency)
  (set `self.People` _outitem)
  (set `/Game/BP_Core/PeopleManagement/BP_Person.Efficiency` (* _efficiency (`self.Efficiency Factor`)) _outitem)
  (`KismetSystemLibrary.PrintString` null "Установлена эффективность рандомному жителю"))