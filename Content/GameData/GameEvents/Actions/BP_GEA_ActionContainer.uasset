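; BP_GEA_ActionContainer is a composite game event action that groups a list of other actions so they act as one.
; Init passes the Holder to each child action, and Deinit tears each one down.
; Enable and Disable call the parent implementation first, then forward the same call to every action in the Actions list.
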(event `self.Init`
  (params (Holder :type "/Game/BP_Core/GameEventManagement/BP_GameEvent Object Reference"))
  (for _array_element (`self.Actions`)
    (`self.Init` _array_element Holder)))

(event `self.Deinit`
  (for _array_element (`self.Actions`)
    (`self.Deinit` _array_element)))

(fn `Disable`
  (`parent.Disable`)
  (for _array_element (`self.Actions`)
    (`self.Disable` _array_element)))

(fn `Enable`
  (`parent.Enable`)
  (for _array_element (`self.Actions`)
    (`self.Enable` _array_element)))