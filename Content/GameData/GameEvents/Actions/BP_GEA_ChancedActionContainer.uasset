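; A game event action container that enables at most one of its child actions by chance.
; Init and Deinit pass through to every action in the Actions array.
; Enable rolls one float from 0 to 1 and enables the first action whose Chance plus AccumulatedChance exceeds it, though AccumulatedChance is never incremented here.
; The chosen action is stored as EnabledAction, which Disable later disables and clears.
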(event `self.Init`
  (params (Holder :type "/Game/BP_Core/GameEventManagement/BP_GameEvent Object Reference"))
  (`parent.Init` Holder)
  (for _array_element (`self.Actions`)
    (`self.Init` (break `/Game/GameData/GameEvents/Actions/S_GEA_ActionAndChance` _array_element) Holder)))

(event `self.Deinit`
  (`parent.Deinit`)
  (for _array_element (`self.Actions`)
    (`self.Deinit` (break `/Game/GameData/GameEvents/Actions/S_GEA_ActionAndChance` _array_element))))

(fn `Disable`
  (bind _enabled_action (`self.Enabled Action`))
  (`parent.Disable`)
  (`/Engine/EditorBlueprintResources/StandardMacros.IsValid` _enabled_action
    (:`Is Valid`
      (`self.Disable` _enabled_action)
      (set `self.Enabled Action` null))))

(fn `Enable`
  (locals (`Accumulated Chance` :type "Float (double-precision)") (Random :type "Float (double-precision)"))
  (`parent.Enable`)
  (set `local.Random` (`KismetMathLibrary.RandomFloatInRange` 0.0 1.0))
  (for _array_element (`self.Actions`)
    (if (< (`local.Random`) (+ (`local.Accumulated Chance`) (`.Chance_4_A64BD77B4FC44BC8EDEF2A8231796A3F` (break `/Game/GameData/GameEvents/Actions/S_GEA_ActionAndChance` _array_element))))
      (`self.Enable` (break `/Game/GameData/GameEvents/Actions/S_GEA_ActionAndChance` _array_element))
      (set `self.Enabled Action` (break `/Game/GameData/GameEvents/Actions/S_GEA_ActionAndChance` _array_element))
      (return))))