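; Game event action that sends a set number of random people to rest for a configured duration.
; On enable, it loops, sampling the person manager's list, and counts only samples whose profession class is BP_RestProfession.
; Each counted pass fires a person from work and assigns them to the rest profession.
; The random pick is re-evaluated after the check, so the person moved can differ from the one tested.
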(fn `Enable`
  (locals (I :type Integer) (Person :type "/Game/BP_Core/PeopleManagement/BP_Person Object Reference"))
  (bind _gamemanager (`/Game/BP_Core/Base/BaseManager.GameManager` (`/Game/BP_Core/GameEventManagement/BP_GameEvent.Event Manager` (`self.Holder Event`))))
  (bind _outitem (`KismetArrayLibrary.Array_Random` (`/Game/BP_Core/PeopleManagement/BP_PersonManager.People` (`/Game/BP_Core/BP_Gamemode.GPersonManager` _gamemanager))))
  (`parent.Enable`)
  (while (< (`local.I`) (`self.Number of People`))
    (if (== (`GameplayStatics.GetObjectClass` (`/Game/BP_Core/PeopleManagement/BP_Person.Profession` _outitem)) "/Game/GameData/Professions/BP_RestProfession.BP_RestProfession_C")
      (`/Engine/EditorBlueprintResources/StandardMacros.IncrementInt` (`local.I`)
        (:`  `
          (bind _output_get (set `local.Person` _outitem))
          (`/Game/BP_Core/PeopleManagement/BP_Person.FireFromWork` _output_get)
          (`/Game/GameData/Professions/BP_RestProfession.Assign Worker` (cast `/Game/GameData/Professions/BP_RestProfession` (`BlueprintMapLibrary.Map_Find` (`/Game/BP_Core/ProfessionManagement/BP_ProfessionManager.Professions` (`/Game/BP_Core/BP_Gamemode.GProfessionsManager` _gamemanager)) "/Game/GameData/Professions/BP_RestProfession.BP_RestProfession_C") :!pure true) _output_get (`self.Rest Duration`)))))))