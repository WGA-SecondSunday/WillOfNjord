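; Base game event for "people lost", which takes people out of availability by sending them to rest for a set duration.
; On Init it builds two people-available conditions, one checking the first amount and one the second, rather than their total.
; It then adds two matching rest actions, each with its own amount and duration, before calling the parent Init with the event manager.
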(event `self.Init`
  (params (`Event Manager` :type "/Game/BP_Core/GameEventManagement/BP_GameEventManager Object Reference"))
  (bind _conditions (`self.Conditions`))
  (`|ExecutionSequence`
    (:`then_0`
      (bind _returnvalue (`|GenericCreateObject` "/Game/GameData/GameEvents/Conditions/BP_GEC_PeopleAmountAvailable.BP_GEC_PeopleAmountAvailable_C" self (`self.First Amount`)))
      (`KismetArrayLibrary.Array_Add` _conditions _returnvalue)
      (bind _returnvalue_2 (`|GenericCreateObject` "/Game/GameData/GameEvents/Conditions/BP_GEC_PeopleAmountAvailable.BP_GEC_PeopleAmountAvailable_C" self (`self.Second Amount`)))
      (`KismetArrayLibrary.Array_Add` _conditions _returnvalue_2))
    (:`then_1`
      (`|ExecutionSequence`
        (:`then_0`
          (bind _returnvalue_3 (`|GenericCreateObject` "/Game/GameData/GameEvents/Actions/BP_GEA_AnyPeopleToRest.BP_GEA_AnyPeopleToRest_C" self (`self.First Amount`) (`self.First Duration`)))
          (`KismetArrayLibrary.Array_Add` (`self.Actions`) (make `/Game/BP_Core/GameEventManagement/S_ActionAndDuration` _returnvalue_3)))
        (:`then_1`
          (bind _returnvalue_4 (`|GenericCreateObject` "/Game/GameData/GameEvents/Actions/BP_GEA_AnyPeopleToRest.BP_GEA_AnyPeopleToRest_C" self (`self.Second Amount`) (`self.Second Duration`)))
          (`KismetArrayLibrary.Array_Add` (`self.Actions`) (make `/Game/BP_Core/GameEventManagement/S_ActionAndDuration` _returnvalue_4)))))
    (:`then_2`
      (`parent.Init` `Event Manager`))))