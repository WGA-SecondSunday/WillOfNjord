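; Base game event prototype for a resource request, offering a take-resource action and a do-nothing action.
; On Init it constructs a TakeResource action from its Resource and Amount variables, then a DoNothing action, both owned by the event.
; Both are appended to the Actions list before the parent Init runs with the event manager.
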(event `self.Init`
  (params (`Event Manager` :type "/Game/BP_Core/GameEventManagement/BP_GameEventManager Object Reference"))
  (`|ExecutionSequence`
    (:`then_0`
      (bind _returnvalue (`|GenericCreateObject` "/Game/GameData/GameEvents/Actions/BP_GEA_TakeResource.BP_GEA_TakeResource_C" self (`self.Resource`) (`self.Amount`)))
      (`KismetArrayLibrary.Array_Add` (`self.Actions`) (make `/Game/BP_Core/GameEventManagement/S_ActionAndDuration` _returnvalue)))
    (:`then_1`
      (bind _returnvalue_2 (`|GenericCreateObject` "/Game/GameData/GameEvents/Actions/BP_GEA_DoNothing.BP_GEA_DoNothing_C" self))
      (`KismetArrayLibrary.Array_Add` (`self.Actions`) (make `/Game/BP_Core/GameEventManagement/S_ActionAndDuration` _returnvalue_2)))
    (:`then_2`
      (`parent.Init` `Event Manager`))))