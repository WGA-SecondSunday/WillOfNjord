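; BP_GEBase_Research is a base game event for research, where researchers of a given profession may earn a resource reward.
; Init adds a workers-available condition, then builds three options: base, enlarged and do nothing, before calling parent Init.
; Both research options pair a chance-based, deferred resource grant with sending researchers to rest, using their own luck chance and duration.
; Conditions and actions are composed at runtime from constructed, nested action objects.
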(event `self.Init`
  (params (`Event Manager` :type "/Game/BP_Core/GameEventManagement/BP_GameEventManager Object Reference"))
  (`|ExecutionSequence`
    (:`then_0`
      (`|ExecutionSequence`
        (:`then_0`
          (bind _returnvalue (`|GenericCreateObject` "/Game/GameData/GameEvents/Conditions/BP_GEC_WorkersAvailable.BP_GEC_WorkersAvailable_C" self (`self.Profession`) (`self.Researchers Count`)))
          (`KismetArrayLibrary.Array_Add` (`self.Conditions`) _returnvalue))))
    (:`then_1`
      (`|ExecutionSequence`
        (:`then_0`
          (bind _returnvalue_2 (`|GenericCreateObject` "/Game/GameData/GameEvents/Actions/BP_GEA_ActionContainer.BP_GEA_ActionContainer_C" self))
          (bind _returnvalue_3 (`|GenericCreateObject` "/Game/GameData/GameEvents/Actions/BP_GEA_ChancedActionContainer.BP_GEA_ChancedActionContainer_C" self))
          (bind _returnvalue_4 (`|GenericCreateObject` "/Game/GameData/GameEvents/Actions/BP_GEA_GiveResource.BP_GEA_GiveResource_C" self (`self.Reward Resource`) (`self.Reward Amount`)))
          (bind _returnvalue_5 (`|GenericCreateObject` "/Game/GameData/GameEvents/Actions/BP_GEA_DefferedAction.BP_GEA_DefferedAction_C" self _returnvalue_4))
          (`KismetArrayLibrary.Array_Add` (`/Game/GameData/GameEvents/Actions/BP_GEA_ChancedActionContainer.Actions` _returnvalue_3) (make `/Game/GameData/GameEvents/Actions/S_GEA_ActionAndChance` _returnvalue_5 (`self.Base Luck Chance`)))
          (bind _actions (`/Game/GameData/GameEvents/Actions/BP_GEA_ActionContainer.Actions` _returnvalue_2))
          (`KismetArrayLibrary.Array_Add` _actions _returnvalue_3)
          (bind _returnvalue_6 (`|GenericCreateObject` "/Game/GameData/GameEvents/Actions/BP_GEA_PeopleToRest.BP_GEA_PeopleToRest_C" self (`self.Profession`) (`self.Base Duration`) (`self.Researchers Count`)))
          (`KismetArrayLibrary.Array_Add` _actions _returnvalue_6)
          (`KismetArrayLibrary.Array_Add` (`self.Actions`) (make `/Game/BP_Core/GameEventManagement/S_ActionAndDuration` _returnvalue_2 (`self.Base Duration`))))
        (:`then_1`
          (bind _returnvalue_7 (`|GenericCreateObject` "/Game/GameData/GameEvents/Actions/BP_GEA_ActionContainer.BP_GEA_ActionContainer_C" self))
          (bind _returnvalue_8 (`|GenericCreateObject` "/Game/GameData/GameEvents/Actions/BP_GEA_ChancedActionContainer.BP_GEA_ChancedActionContainer_C" self))
          (bind _returnvalue_9 (`|GenericCreateObject` "/Game/GameData/GameEvents/Actions/BP_GEA_GiveResource.BP_GEA_GiveResource_C" self (`self.Reward Resource`) (`self.Reward Amount`)))
          (bind _returnvalue_10 (`|GenericCreateObject` "/Game/GameData/GameEvents/Actions/BP_GEA_DefferedAction.BP_GEA_DefferedAction_C" self _returnvalue_9))
          (`KismetArrayLibrary.Array_Add` (`/Game/GameData/GameEvents/Actions/BP_GEA_ChancedActionContainer.Actions` _returnvalue_8) (make `/Game/GameData/GameEvents/Actions/S_GEA_ActionAndChance` _returnvalue_10 (`self.Enlarged Luck Chance`)))
          (bind _actions_2 (`/Game/GameData/GameEvents/Actions/BP_GEA_ActionContainer.Actions` _returnvalue_7))
          (`KismetArrayLibrary.Array_Add` _actions_2 _returnvalue_8)
          (bind _returnvalue_11 (`|GenericCreateObject` "/Game/GameData/GameEvents/Actions/BP_GEA_PeopleToRest.BP_GEA_PeopleToRest_C" self (`self.Profession`) (`self.Enlarged Duration`) (`self.Researchers Count`)))
          (`KismetArrayLibrary.Array_Add` _actions_2 _returnvalue_11)
          (`KismetArrayLibrary.Array_Add` (`self.Actions`) (make `/Game/BP_Core/GameEventManagement/S_ActionAndDuration` _returnvalue_7 (`self.Enlarged Duration`))))
        (:`then_2`
          (bind _returnvalue_12 (`|GenericCreateObject` "/Game/GameData/GameEvents/Actions/BP_GEA_DoNothing.BP_GEA_DoNothing_C" self))
          (`KismetArrayLibrary.Array_Add` (`self.Actions`) (make `/Game/BP_Core/GameEventManagement/S_ActionAndDuration` _returnvalue_12)))))
    (:`then_2`
      (`parent.Init` `Event Manager`))))