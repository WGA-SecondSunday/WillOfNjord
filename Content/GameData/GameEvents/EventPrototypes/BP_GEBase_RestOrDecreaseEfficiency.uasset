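; Base game event prototype that sends random people to rest and applies a temporary efficiency factor to random people.
; On Init it builds a condition that enough people are available for the rest amount.
; It then registers two actions, the rest and the efficiency change, the latter paired with its promotion duration, before calling parent Init.
; Despite "DecreaseEfficiency" in the asset name, the factor variable is named as an increase.
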(event `self.Init`
  (params (`Event Manager` :type "/Game/BP_Core/GameEventManagement/BP_GameEventManager Object Reference"))
  (`|ExecutionSequence`
    (:`then_0`
      (bind _returnvalue (`|GenericCreateObject` "/Game/GameData/GameEvents/Conditions/BP_GEC_PeopleAmountAvailable.BP_GEC_PeopleAmountAvailable_C" self (`self.Rest People Amount`)))
      (`KismetArrayLibrary.Array_Add` (`self.Conditions`) _returnvalue))
    (:`then_1`
      (`|ExecutionSequence`
        (:`then_0`
          (bind _returnvalue_2 (`|GenericCreateObject` "/Game/GameData/GameEvents/Actions/BP_GEA_RandomPeopleToRest.BP_GEA_RandomPeopleToRest_C" self (`self.Rest Duration`) (`self.Rest People Amount`)))
          (`KismetArrayLibrary.Array_Add` (`self.Actions`) (make `/Game/BP_Core/GameEventManagement/S_ActionAndDuration` _returnvalue_2)))
        (:`then_1`
          (bind _returnvalue_3 (`|GenericCreateObject` "/Game/GameData/GameEvents/Actions/BP_GEA_RandomPeopleSetTempEfficiency.BP_GEA_RandomPeopleSetTempEfficiency_C" self (`self.Efficiency Increase Factor`)))
          (`KismetArrayLibrary.Array_Add` (`self.Actions`) (make `/Game/BP_Core/GameEventManagement/S_ActionAndDuration` _returnvalue_3 (`self.Efficiency Promotion Duration`))))))
    (:`then_2`
      (`parent.Init` `Event Manager`))))