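; BP_GEBase_Accident is a base game event for accidents that send workers to rest.
; Init adds worker-availability conditions for a primary and a secondary profession, then builds two action entries before calling the parent Init.
; The first entry rests the primary workers for their full rest time.
; The second uses an action container to rest primary workers for half that time and secondary workers for their own rest time.
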(event `self.Init`
  (params (`Event Manager` :type "/Game/BP_Core/GameEventManagement/BP_GameEventManager Object Reference"))
  (bind _conditions (`self.Conditions`))
  (`|ExecutionSequence`
    (:`then_0`
      (`|ExecutionSequence`
        (:`then_0`
          (bind _returnvalue (`|GenericCreateObject` "/Game/GameData/GameEvents/Conditions/BP_GEC_WorkersAvailable.BP_GEC_WorkersAvailable_C" self (`self.Primary Profession`) (`self.Primary People Count`)))
          (`KismetArrayLibrary.Array_Add` _conditions _returnvalue)
          (bind _returnvalue_2 (`|GenericCreateObject` "/Game/GameData/GameEvents/Conditions/BP_GEC_WorkersAvailable.BP_GEC_WorkersAvailable_C" self (`self.Secondary Profession`) (`self.Secondary People Count`)))
          (`KismetArrayLibrary.Array_Add` _conditions _returnvalue_2))))
    (:`then_1`
      (`|ExecutionSequence`
        (:`then_0`
          (bind _returnvalue_3 (`|GenericCreateObject` "/Game/GameData/GameEvents/Actions/BP_GEA_PeopleToRest.BP_GEA_PeopleToRest_C" self (`self.Primary Profession`) (`self.Primary Rest Time`) (`self.Primary People Count`)))
          (`KismetArrayLibrary.Array_Add` (`self.Actions`) (make `/Game/BP_Core/GameEventManagement/S_ActionAndDuration` _returnvalue_3)))
        (:`then_1`
          (bind _returnvalue_4 (`|GenericCreateObject` "/Game/GameData/GameEvents/Actions/BP_GEA_ActionContainer.BP_GEA_ActionContainer_C" self))
          (bind _returnvalue_5 (`|GenericCreateObject` "/Game/GameData/GameEvents/Actions/BP_GEA_PeopleToRest.BP_GEA_PeopleToRest_C" self (`self.Primary Profession`) (`/Game/BP_Core/TimeManagement/BP_TimeFuncs.Game Time Div` (`self.Primary Rest Time`) 2) (`self.Primary People Count`)))
          (bind _actions (`/Game/GameData/GameEvents/Actions/BP_GEA_ActionContainer.Actions` _returnvalue_4))
          (`KismetArrayLibrary.Array_Add` _actions _returnvalue_5)
          (bind _returnvalue_6 (`|GenericCreateObject` "/Game/GameData/GameEvents/Actions/BP_GEA_PeopleToRest.BP_GEA_PeopleToRest_C" self (`self.Secondary Profession`) (`self.Secondary Rest Time`) (`self.Secondary People Count`)))
          (`KismetArrayLibrary.Array_Add` _actions _returnvalue_6)
          (`/Game/BP_Core/GameEventManagement/BP_GameEventAction.Init` _returnvalue_4 self)
          (`KismetArrayLibrary.Array_Add` (`self.Actions`) (make `/Game/BP_Core/GameEventManagement/S_ActionAndDuration` _returnvalue_4)))))
    (:`then_2`
      (`parent.Init` `Event Manager`))))