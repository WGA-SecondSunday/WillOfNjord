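; Base game event prototype that offers two outcomes: send workers of a profession to rest, or rest them and take a resource.
; Init adds a workers-available condition sized to the larger of the two people amounts.
; It builds a plain rest action and a container pairing a second rest action with a percentage-based resource take.
; The parent Init runs after conditions and actions are registered.
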(event `self.Init`
  (params (`Event Manager` :type "/Game/BP_Core/GameEventManagement/BP_GameEventManager Object Reference"))
  (`|ExecutionSequence`
    (:`then_0`
      (bind _returnvalue (`|GenericCreateObject` "/Game/GameData/GameEvents/Conditions/BP_GEC_WorkersAvailable.BP_GEC_WorkersAvailable_C" self (`self.Affected Profession`) (`KismetMathLibrary.Max` (`self.First People Amount`) (`self.Second People Amount`))))
      (`KismetArrayLibrary.Array_Add` (`self.Conditions`) _returnvalue))
    (:`then_1`
      (`|ExecutionSequence`
        (:`then_0`
          (bind _returnvalue_2 (`|GenericCreateObject` "/Game/GameData/GameEvents/Actions/BP_GEA_PeopleToRest.BP_GEA_PeopleToRest_C" self (`self.Affected Profession`) (`self.First Rest Duration`) (`self.First People Amount`)))
          (`KismetArrayLibrary.Array_Add` (`self.Actions`) (make `/Game/BP_Core/GameEventManagement/S_ActionAndDuration` _returnvalue_2)))
        (:`then_1`
          (`|ExecutionSequence`
            (:`then_0`
              (bind _returnvalue_3 (`|GenericCreateObject` "/Game/GameData/GameEvents/Actions/BP_GEA_ActionContainer.BP_GEA_ActionContainer_C" self))
              (bind _returnvalue_4 (`|GenericCreateObject` "/Game/GameData/GameEvents/Actions/BP_GEA_PeopleToRest.BP_GEA_PeopleToRest_C" self (`self.Affected Profession`) (`self.Second Rest Duration`) (`self.Second People Amount`)))
              (bind _actions (`/Game/GameData/GameEvents/Actions/BP_GEA_ActionContainer.Actions` _returnvalue_3))
              (`KismetArrayLibrary.Array_Add` _actions _returnvalue_4)
              (bind _returnvalue_5 (`|GenericCreateObject` "/Game/GameData/GameEvents/Actions/BP_GEA_TakeResourceByPercentage.BP_GEA_TakeResourceByPercentage_C" self (`self.Resource`) (`self.Resource Amount Percentage`)))
              (`KismetArrayLibrary.Array_Add` _actions _returnvalue_5))
            (:`then_1`
              (`KismetArrayLibrary.Array_Add` (`self.Actions`) (make `/Game/BP_Core/GameEventManagement/S_ActionAndDuration` _returnvalue_3)))))))
    (:`then_2`
      (`parent.Init` `Event Manager`))))