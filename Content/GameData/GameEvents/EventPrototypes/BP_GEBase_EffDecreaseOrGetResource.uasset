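; Base game event that either temporarily lowers worker efficiency or grants a resource, as its name indicates.
; On Init it adds a condition requiring an available worker of the configured profession, then builds two actions before calling the parent Init.
; The first is a chanced container pairing the efficiency penalty at a configurable chance with a resource reward at full chance, registered with the decrease duration.
; The second action does nothing.
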(event `self.Init`
  (params (`Event Manager` :type "/Game/BP_Core/GameEventManagement/BP_GameEventManager Object Reference"))
  (`|ExecutionSequence`
    (:`then_0`
      (bind _returnvalue (`|GenericCreateObject` "/Game/GameData/GameEvents/Conditions/BP_GEC_WorkersAvailable.BP_GEC_WorkersAvailable_C" self (`self.Profession`) 1))
      (`KismetArrayLibrary.Array_Add` (`self.Conditions`) _returnvalue))
    (:`then_1`
      (`|ExecutionSequence`
        (:`then_0`
          (bind _returnvalue_2 (`|GenericCreateObject` "/Game/GameData/GameEvents/Actions/BP_GEA_ChancedActionContainer.BP_GEA_ChancedActionContainer_C" self))
          (bind _returnvalue_3 (`|GenericCreateObject` "/Game/GameData/GameEvents/Actions/BP_GEA_RandomPeopleSetTempEfficiency.BP_GEA_RandomPeopleSetTempEfficiency_C" self (`self.Eff Decrease Factor`)))
          (bind _actions (`/Game/GameData/GameEvents/Actions/BP_GEA_ChancedActionContainer.Actions` _returnvalue_2))
          (`KismetArrayLibrary.Array_Add` _actions (make `/Game/GameData/GameEvents/Actions/S_GEA_ActionAndChance` _returnvalue_3 (`self.Decrease Chance`)))
          (bind _returnvalue_4 (`|GenericCreateObject` "/Game/GameData/GameEvents/Actions/BP_GEA_GiveResource.BP_GEA_GiveResource_C" self (`self.Reward Resource`) (`self.Reward Amount`)))
          (`KismetArrayLibrary.Array_Add` _actions (make `/Game/GameData/GameEvents/Actions/S_GEA_ActionAndChance` _returnvalue_4 100.0))
          (`KismetArrayLibrary.Array_Add` (`self.Actions`) (make `/Game/BP_Core/GameEventManagement/S_ActionAndDuration` _returnvalue_2 (`self.Decrease Duration`))))
        (:`then_1`
          (bind _returnvalue_5 (`|GenericCreateObject` "/Game/GameData/GameEvents/Actions/BP_GEA_DoNothing.BP_GEA_DoNothing_C" self))
          (`KismetArrayLibrary.Array_Add` (`self.Actions`) (make `/Game/BP_Core/GameEventManagement/S_ActionAndDuration` _returnvalue_5)))))
    (:`then_2`
      (`parent.Init` `Event Manager`))))