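; Base prototype for a game event that temporarily buffs a profession's efficiency.
; On Init it builds a condition requiring one available worker of the configured profession.
; It also builds an action that raises that profession's efficiency by the configured amount, registered with a duration, then calls the parent Init.
; Subclasses presumably only need to set profession, efficiency and duration.
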(event `self.Init`
  (params (`Event Manager` :type "/Game/BP_Core/GameEventManagement/BP_GameEventManager Object Reference"))
  (`|ExecutionSequence`
    (:`then_0`
      (bind _returnvalue (`|GenericCreateObject` "/Game/GameData/GameEvents/Conditions/BP_GEC_WorkersAvailable.BP_GEC_WorkersAvailable_C" self (`self.Profession`) 1))
      (`KismetArrayLibrary.Array_Add` (`self.Conditions`) _returnvalue))
    (:`then_1`
      (bind _returnvalue_2 (`|GenericCreateObject` "/Game/GameData/GameEvents/Actions/BP_GEA_RaiseProfessionEfficiencyTemporarily.BP_GEA_RaiseProfessionEfficiencyTemporarily_C" self (`self.Profession`) (`self.Applied Efficiency`)))
      (`KismetArrayLibrary.Array_Add` (`self.Actions`) (make `/Game/BP_Core/GameEventManagement/S_ActionAndDuration` _returnvalue_2 (`self.Duration`))))
    (:`then_2`
      (`parent.Init` `Event Manager`))))