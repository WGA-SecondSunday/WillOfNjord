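; Base game event prototype for a neighbour disturbance that debuffs a profession and moves one person without a profession into the warriors.
; On Init it constructs two action objects: a temporary profession efficiency change, driven by configurable profession, efficiency and duration values, and a reassignment.
; It adds both to the Actions list, then calls the parent Init; it adds no conditions of its own.
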(event `self.Init`
  (params (`Event Manager` :type "/Game/BP_Core/GameEventManagement/BP_GameEventManager Object Reference"))
  (`|ExecutionSequence`
    (:`then_1`
      (`|ExecutionSequence`
        (:`then_0`
          (bind _returnvalue (`|GenericCreateObject` "/Game/GameData/GameEvents/Actions/BP_GEA_RaiseProfessionEfficiencyTemporarily.BP_GEA_RaiseProfessionEfficiencyTemporarily_C" self (`self.Profession To Debuff`) (`self.Debuff Efficiency`)))
          (`KismetArrayLibrary.Array_Add` (`self.Actions`) (make `/Game/BP_Core/GameEventManagement/S_ActionAndDuration` _returnvalue (`self.Debuff Duration`))))
        (:`then_1`
          (bind _returnvalue_2 (`|GenericCreateObject` "/Game/GameData/GameEvents/Actions/BP_GEA_ReassignProfessions.BP_GEA_ReassignProfessions_C" self "/Game/GameData/Professions/BP_NoProfession.BP_NoProfession_C" "/Game/GameData/Professions/BP_Warriors.BP_Warriors_C" 1))
          (`KismetArrayLibrary.Array_Add` (`self.Actions`) (make `/Game/BP_Core/GameEventManagement/S_ActionAndDuration` _returnvalue_2)))))
    (:`then_2`
      (`parent.Init` `Event Manager`))))