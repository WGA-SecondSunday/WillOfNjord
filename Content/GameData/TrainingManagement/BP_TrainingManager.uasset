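; Training manager that runs a step-by-step tutorial once GameManager reports the game is initialized.
; Steps form a class-linked chain from BeginningStep: Proceed clears hints, deinitializes the current step, then constructs and initializes its NextStep.
; CreateHint builds hint widgets from step settings and binds their Next and Close buttons.
; SkipTraining disables hints and fast-forwards through remaining steps, completing each before exiting training mode.
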(event `self.ReceiveBeginPlay`
  (`parent.ReceiveBeginPlay`)
  (add `/Game/BP_Core/BP_Gamemode.GameInitialized` (`self.GameManager`) (delegate `CustomEvent_0`)))

(event `CustomEvent_0`
  (`self.Proceed` true))

(fn `Create Hint`
  (params (Step :type "/Game/GameData/TrainingManagement/BP_TrainingStepBase Object Reference"))
  (returns (Hint :type "/Game/UI/Widgets/HintWidget/BP_HintWidget Object Reference"))
  (bind _returnvalue (`|CreateWidget` "/Game/UI/Widgets/HintWidget/BP_HintWidget.BP_HintWidget_C" null (`/Game/GameData/TrainingManagement/BP_TrainingStepBase.Next Enabled` Step) (`/Game/GameData/TrainingManagement/BP_TrainingStepBase.Close Enabled` Step) (`/Game/GameData/TrainingManagement/BP_TrainingStepBase.Hint Size` Step) (`/Game/GameData/TrainingManagement/BP_TrainingStepBase.Hint Position` Step) (`/Game/GameData/TrainingManagement/BP_TrainingStepBase.Hint Text` Step)))
  (add `Button.OnClicked` (`/Game/UI/Widgets/HintWidget/BP_HintWidget.CloseBtn` _returnvalue) (`|CreateDelegate` :!event `Skip Training`))
  (add `Button.OnClicked` (`/Game/UI/Widgets/HintWidget/BP_HintWidget.NextBtn` _returnvalue) (`|CreateDelegate` :!event `Proceed To Next Step`))
  (return _returnvalue))

(fn `Exit From Training Mode`
  (set `self.Current Step` null)
  (`KismetSystemLibrary.PrintString` "Обучение закончено 2"))

(fn `Proceed`
  (params (`Is First` :type Boolean))
  (bind _current_step (`self.Current Step`))
  (bind _next_step (`/Game/GameData/TrainingManagement/BP_TrainingStepBase.Next Step` _current_step))
  (if `Is First`
    (bind _returnvalue (`|GenericCreateObject` (`self.Beginning Step`) self self))
    (bind _output_get (set `self.Current Step` _returnvalue))
    (`/Game/GameData/TrainingManagement/BP_TrainingStepBase.Init` _output_get :!label _label)
    (`/Game/GameData/TrainingManagement/BP_TrainingStepBase.Init` (`self.Current Step`))
    (if (`self.Show Hints`)
      (`/Game/GameData/TrainingManagement/BP_TrainingStepBase.Show Hint` (`self.Current Step`)))
    (else
      (`/Engine/EditorBlueprintResources/StandardMacros.IsValid` _current_step
        (:`Is Valid`
          (bind _foundwidgets (`WidgetBlueprintLibrary.GetAllWidgetsOfClass` "/Game/UI/Widgets/HintWidget/BP_HintWidget.BP_HintWidget_C"))
          (for _array_element _foundwidgets
            (`Widget.RemoveFromParent` _array_element))
          (`/Game/GameData/TrainingManagement/BP_TrainingStepBase.Deinit` _current_step)
          (if (`KismetSystemLibrary.IsValidClass` _next_step)
            (bind _returnvalue_2 (`|GenericCreateObject` _next_step self self))
            (set `self.Current Step` _returnvalue_2)
            (goto _label)
            (else
              (`self.Exit From Training Mode`))))))))

(fn `Proceed To Next Step`
  (`self.Proceed` false))

(fn `Skip Training`
  (locals (`Next Step` :type "/Game/GameData/TrainingManagement/BP_TrainingStepBase Class Reference"))
  (bind _current_step (`self.Current Step`))
  (set `self.Show Hints` false)
  (bind _foundwidgets (`WidgetBlueprintLibrary.GetAllWidgetsOfClass` "/Game/UI/Widgets/HintWidget/BP_HintWidget.BP_HintWidget_C" false))
  (for _array_element _foundwidgets
    (`Widget.RemoveFromParent` _array_element))
  (set `local.Next Step` (`/Game/GameData/TrainingManagement/BP_TrainingStepBase.Next Step` (`self.Current Step`)))
  (while (`KismetSystemLibrary.IsValidClass` (`local.Next Step`))
    (`self.Proceed` false)
    (`/Game/GameData/TrainingManagement/BP_TrainingStepBase.Complete` _current_step)
    (set `local.Next Step` (`/Game/GameData/TrainingManagement/BP_TrainingStepBase.Next Step` _current_step)))
  (`self.Exit From Training Mode`))

(fn `UserConstructionScript`
  (`parent.UserConstructionScript`))