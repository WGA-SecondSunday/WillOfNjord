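; Building condition that passes only when every building class tracked in its BuildingsCount map has a non-zero count.
; On Init it binds to the BuildingManager's building status change event.
; Its listener adjusts counts for classes already in the map, incrementing when the new status is above zero and decrementing otherwise, regardless of the old status.
; CheckCondition calls the parent, then returns false on any zero count.
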(event `self.Init`
  (params (`Building Manager` :type "/Game/BP_Core/BuildingManagement/BP_BuildingManager Object Reference"))
  (add `/Game/BP_Core/BuildingManagement/BP_BuildingManager.OnBuildingStatusChanged` `Building Manager` (`|CreateDelegate` :!event `Building Listener`)))

(fn `Building Listener`
  (params (Building :type "/Game/BP_Core/BuildingManagement/BP_Building Object Reference") (`Old Status` :type Integer) (`New Status` :type Integer))
  (bind _returnvalue (`GameplayStatics.GetObjectClass` Building))
  (bind _buildings_count (`self.Buildings Count`))
  (bind (_value _returnvalue_2) (`BlueprintMapLibrary.Map_Find` _buildings_count _returnvalue))
  (if _returnvalue_2
    (if (> `New Status` 0)
      (`BlueprintMapLibrary.Map_Add` _buildings_count _returnvalue (+ _value 1))
      (else
        (`BlueprintMapLibrary.Map_Add` _buildings_count _returnvalue (- _value 1))))))

(fn `CheckCondition`
  (params (Manager :type "/Game/BP_Core/BuildingManagement/BP_BuildingManager Object Reference"))
  (returns (Result :type Boolean))
  (`parent.CheckCondition` Manager)
  (bind _values (`BlueprintMapLibrary.Map_Values` (`self.Buildings Count`)))
  (for _array_element _values
    (if (== _array_element 0)
      (return false)))
  (return true))