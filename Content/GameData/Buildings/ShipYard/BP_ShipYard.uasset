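; BP_ShipYard is the shipyard building, a child of a building base class that overrides its level effect hooks.
; Applying the effect runs the parent logic, then reports the building to the shipyard manager, reached through BuildingsManager and GameManager.
; Cancelling the effect only hides the ship progress widget on the HUD, without calling the parent or notifying the shipyard manager.
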(fn `Apply Effect`
  (params (`New Level` :type Integer))
  (`parent.Apply Effect` `New Level`)
  (`/Game/BP_Core/ShipYardManagement/BP_YardManager.Ship Yard Built Handler` (`/Game/BP_Core/BP_Gamemode.GShipYardManager` (`/Game/BP_Core/Base/BaseManager.GameManager` (`self.Buildings Manager`))) self))

(fn `CancelEffect`
  (params (PrevLevel :type Integer))
  (`Widget.SetVisibility` (`/Game/UI/Widgets/TimerAndScreenButtons/BP_HUD.ShipProgress` (`/Game/BP_Core/BP_Gamemode.WHUD` (`/Game/BP_Core/Base/BaseManager.GameManager` (`self.Buildings Manager`)))) "Hidden"))

(fn `UserConstructionScript`
  (`parent.UserConstructionScript`))