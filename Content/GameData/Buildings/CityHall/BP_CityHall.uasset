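; BP_CityHall is the City Hall building Blueprint, which raises the population cap while its effect is applied.
; Apply Effect adds the first Capacities entry to MaxPeople on the GPersonManager, reached through BuildingsManager and GameManager, and CancelEffect subtracts it.
; Both functions ignore their level argument and always use that first entry.
; The event graph has no active logic.
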(fn `Apply Effect`
  (params (`New Level` :type Integer))
  (bind _gpersonmanager (`/Game/BP_Core/BP_Gamemode.GPersonManager` (`/Game/BP_Core/Base/BaseManager.GameManager` (`self.Buildings Manager`))))
  (set `/Game/BP_Core/PeopleManagement/BP_PersonManager.MaxPeople` (+ (`/Game/BP_Core/PeopleManagement/BP_PersonManager.MaxPeople` _gpersonmanager) (`|GetArrayItem` (`self.Capacities`))) _gpersonmanager))

(fn `CancelEffect`
  (params (PrevLevel :type Integer))
  (bind _gpersonmanager (`/Game/BP_Core/BP_Gamemode.GPersonManager` (`/Game/BP_Core/Base/BaseManager.GameManager` (`self.Buildings Manager`))))
  (set `/Game/BP_Core/PeopleManagement/BP_PersonManager.MaxPeople` (- (`/Game/BP_Core/PeopleManagement/BP_PersonManager.MaxPeople` _gpersonmanager) (`|GetArrayItem` (`self.Capacities`))) _gpersonmanager))

(fn `UserConstructionScript`
  (`parent.UserConstructionScript`))