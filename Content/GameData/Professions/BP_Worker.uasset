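; Worker profession that drives building construction through a time resource.
; On init it registers a producer entry, then once the game initializes it binds to new building tasks and to the time resource's goal event.
; A new task takes the front of the building queue and sets the resource goal to its status change time in minutes.
; Reaching the goal ends that building's status update and zeroes the resource's amount and goal.
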(event `self.Init`
  (params (Manager :type "/Game/BP_Core/ProfessionManagement/BP_ProfessionManager Object Reference"))
  (`parent.Init` Manager)
  (add `/Game/BP_Core/BP_Gamemode.GameInitialized` (`/Game/BP_Core/Base/BaseManager.GameManager` Manager) (delegate `Initialized`))
  (`KismetArrayLibrary.Array_Add` (`self.Producers`) (make `/Game/BP_Core/ProfessionManagement/BP_Producer` "NewEnumerator6" 1.0 10.0)))

(event `Initialized`
  (bind _gamemanager (`/Game/BP_Core/Base/BaseManager.GameManager` (stale `self.Init` Manager)))
  (bind _output_get (set `self.Building Manager` (`/Game/BP_Core/BP_Gamemode.GBuildingManager` _gamemanager)))
  (add `/Game/BP_Core/BuildingManagement/BP_BuildingManager.OnNewBuildingTask` _output_get (`|CreateDelegate` :!event `Handle New Building Task`))
  (bind _output_get_2 (set `self.Time Resource` (`BlueprintMapLibrary.Map_Find` (`/Game/BP_Core/ResourceManagement/BP_UResourceManager.Resources` (`/Game/BP_Core/BP_Gamemode.GResourceManager` _gamemanager)) "NewEnumerator6")))
  (add `/Game/BP_Core/ResourceManagement/BP_UResource.OnGoalReached` _output_get_2 (`|CreateDelegate` :!event `Goal Reached`)))

(fn `Goal Reached`
  (params (Resource :type "/Game/BP_Core/ResourceManagement/BP_UResource Object Reference"))
  (bind _time_resource (`self.Time Resource`))
  (`/Game/BP_Core/BuildingManagement/BP_Building.EndStatusUpdate` (`self.Constructing Building`))
  (`/Game/BP_Core/ResourceManagement/BP_UResource.UpdateAmount` _time_resource 0.0)
  (`/Game/BP_Core/ResourceManagement/BP_UResource.Update Goal` _time_resource 0.0))

(fn `Handle New Building Task`
  (bind _building_queue (`/Game/BP_Core/BuildingManagement/BP_BuildingManager.Building Queue` (`self.Building Manager`)))
  (bind _output (`|GetArrayItem` _building_queue))
  (set `self.Constructing Building` _output)
  (if (> (`KismetArrayLibrary.Array_Length` _building_queue) 0)
    (`/Game/BP_Core/ResourceManagement/BP_UResource.Update Goal` (`self.Time Resource`) (`KismetMathLibrary.Conv_IntToDouble` (`/Game/BP_Core/TimeManagement/BP_TimeManager.GTime to Minutes` (`/Game/BP_Core/BP_Gamemode.GTimeManager` (`/Game/BP_Core/Base/BaseManager.GameManager` (`self.Manager`))) (`/Game/BP_Core/BuildingManagement/BP_Building.Status Change Time` _output))))))