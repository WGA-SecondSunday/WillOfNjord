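; BP_Warriors is a profession Blueprint that adds defence to the game's resources while warriors are assigned.
; Its MakeWork function runs only when it has at least one worker, finds an enum-keyed entry in the resource manager's map, and updates its amount by DefenceAmountPerHour.
; The gain is a flat amount, not scaled by the number of workers.
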(fn `MakeWork`
  (params (ResMan :type "/Game/BP_Core/ResourceManagement/BP_UResourceManager Object Reference (by ref)"))
  (bind _value (`BlueprintMapLibrary.Map_Find` (`/Game/BP_Core/ResourceManagement/BP_UResourceManager.Resources` ResMan) "NewEnumerator10"))
  (if (> (`KismetArrayLibrary.Array_Length` (`self.Workers`)) 0)
    (`/Game/BP_Core/ResourceManagement/BP_UResource.UpdateAmount` _value (+ (`/Game/BP_Core/ResourceManagement/BP_UResource.Amount` _value) (`self.Defence Amount Per Hour`)))
    (return)))