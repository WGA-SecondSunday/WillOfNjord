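; BP_RestProfession is a profession that holds resting people as workers for a limited time.
; Assigning a worker creates a timer through the game's time manager, stores it on the person, then runs the standard worker assignment without bypassing the maximum amount.
; The timer handler searches the workers for the person whose rest timer matches and fires them from work, ending the rest.
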(fn `Assign Worker`
  (params (Person :type "/Game/BP_Core/PeopleManagement/BP_Person Object Reference (by ref)") (`Time For Rest` :type "/Game/BP_Core/TimeManagement/BP_GameTime Structure"))
  (bind _timer (`/Game/BP_Core/TimeManagement/BP_TimeManager.Create Timer` (`/Game/BP_Core/BP_Gamemode.GTimeManager` (`/Game/BP_Core/Base/BaseManager.GameManager` (`self.Manager`))) `Time For Rest` (`|CreateDelegate` :!event `Timer Handler`)))
  (set `/Game/BP_Core/PeopleManagement/BP_Person.Rest Timer` _timer Person)
  (`self.AssignWorker` Person))

(fn `Timer Handler`
  (params (Timer :type "/Game/BP_Core/TimeManagement/BP_Timer Object Reference"))
  (for _array_element (`self.Workers`)
    (if (== (`/Game/BP_Core/PeopleManagement/BP_Person.Rest Timer` _array_element) Timer)
      (`/Game/BP_Core/PeopleManagement/BP_Person.FireFromWork` _array_element)
      (return))))