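; Profession blueprint that releases all of its workers from their jobs when the day ends.
; On init it waits for game initialization, then subscribes to the game event manager's event-activated notification.
; When an activated event's class derives from the configured day-ending event, it repeatedly fires the first worker until the worker list is empty.
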(event `self.Init`
  (params (Manager :type "/Game/BP_Core/ProfessionManagement/BP_ProfessionManager Object Reference"))
  (`parent.Init` Manager)
  (add `/Game/BP_Core/BP_Gamemode.GameInitialized` (`/Game/BP_Core/Base/BaseManager.GameManager` Manager) (delegate `CustomEvent_1`)))

(event `CustomEvent_1`
  (add `/Game/BP_Core/GameEventManagement/BP_GameEventManager.OnEventActivated` (`/Game/BP_Core/BP_Gamemode.GGameEventManager` (`/Game/BP_Core/Base/BaseManager.GameManager` (stale `self.Init` Manager))) (delegate `CustomEvent_0`)))

(event `CustomEvent_0`
  (params (Event :type "/Game/BP_Core/GameEventManagement/BP_GameEvent Object Reference"))
  (bind _workers (`self.Workers`))
  (if (`KismetMathLibrary.ClassIsChildOf` (`GameplayStatics.GetObjectClass` Event) (`/Game/BP_Core/GameEventManagement/BPDA_GameEvents.Day Ending Event` (`/Game/BP_Core/GameEventManagement/BP_GameEventManager.Static Data` (`/Game/BP_Core/BP_Gamemode.GGameEventManager` (`/Game/BP_Core/Base/BaseManager.GameManager` (stale `self.Init` Manager))))))
    (while (> (`KismetArrayLibrary.Array_Length` _workers) 0)
      (`/Game/BP_Core/PeopleManagement/BP_Person.FireFromWork` (`|GetArrayItem` _workers)))))