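; Game stage Blueprint for the second stage, which ends when its timer runs out or a shipyard reaches a qualifying status.
; Init creates a stage-duration timer through the time manager and binds to the building manager's status change event.
; Either timer expiry or a BP_ShipYard changing to an even-valued status makes the GameManager transit to the next stage.
; Deinit deletes the timer and unbinds the building event.
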(event `self.Init`
  (params (`Game Manager` :type "/Game/BP_Core/BP_Gamemode Object Reference"))
  (bind _timer (`/Game/BP_Core/TimeManagement/BP_TimeManager.Create Timer` (`/Game/BP_Core/BP_Gamemode.GTimeManager` `Game Manager`) (`self.Stage Duration`) (delegate `CustomEvent_0`)))
  (set `self.Timer` _timer)
  (add `/Game/BP_Core/BuildingManagement/BP_BuildingManager.OnBuildingStatusChanged` (`/Game/BP_Core/BP_Gamemode.GBuildingManager` `Game Manager`) (delegate `CustomEvent_1`))
  (`KismetSystemLibrary.PrintString` null "Second Stage Started"))

(event `CustomEvent_1`
  (params (Building :type "/Game/BP_Core/BuildingManagement/BP_Building Object Reference") (`Old Status` :type Integer) (`New Status` :type Integer))
  (if (and (== (`GameplayStatics.GetObjectClass` Building) "/Game/GameData/Buildings/ShipYard/BP_ShipYard.BP_ShipYard_C") (== (mod `New Status` 2) 0))
    (`/Game/BP_Core/BP_Gamemode.Transit To Stage` (stale `self.Init` `Game Manager`) (`self.Next Stage`))))

(event `CustomEvent_0`
  (params (Timer :type "/Game/BP_Core/TimeManagement/BP_Timer Object Reference"))
  (`/Game/BP_Core/BP_Gamemode.Transit To Stage` (stale `self.Init` `Game Manager`) (`self.Next Stage`)))

(event `self.Deinit`
  (params (`Game Manager` :type "/Game/BP_Core/BP_Gamemode Object Reference"))
  (`/Game/BP_Core/TimeManagement/BP_TimeManager.Delete Timer` (`/Game/BP_Core/BP_Gamemode.GTimeManager` `Game Manager`) (`self.Timer`))
  (remove `/Game/BP_Core/BuildingManagement/BP_BuildingManager.OnBuildingStatusChanged` (`/Game/BP_Core/BP_Gamemode.GBuildingManager` `Game Manager`) (delegate `CustomEvent_1`))
  (`KismetSystemLibrary.PrintString` null "Second Stage Ended"))