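; BP_InitialStage is a timed game stage, apparently the opening one, that hands off to a next stage after a set duration.
; On Init it creates a timer of StageDuration through the GameManager's GTimeManager.
; When that timer ends, its callback asks the GameManager to transit to NextStage.
; Deinit deletes the timer, and both Init and Deinit print a debug message.
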(event `self.Init`
  (params (`Game Manager` :type "/Game/BP_Core/BP_Gamemode Object Reference"))
  (bind _timer (`/Game/BP_Core/TimeManagement/BP_TimeManager.Create Timer` (`/Game/BP_Core/BP_Gamemode.GTimeManager` `Game Manager`) (`self.Stage Duration`) (delegate `CustomEvent_0`)))
  (set `self.Timer` _timer)
  (`KismetSystemLibrary.PrintString` null "Initial Stage Started"))

(event `CustomEvent_0`
  (params (Timer :type "/Game/BP_Core/TimeManagement/BP_Timer Object Reference"))
  (`/Game/BP_Core/BP_Gamemode.Transit To Stage` (stale `self.Init` `Game Manager`) (`self.Next Stage`)))

(event `self.Deinit`
  (params (`Game Manager` :type "/Game/BP_Core/BP_Gamemode Object Reference"))
  (`/Game/BP_Core/TimeManagement/BP_TimeManager.Delete Timer` (`/Game/BP_Core/BP_Gamemode.GTimeManager` `Game Manager`) (`self.Timer`))
  (`KismetSystemLibrary.PrintString` null "Initial Stage Ended"))