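; Base game stage Blueprint that swaps in the stage's set of game events and opens the stage with a custom titled event.
; Load clears the event manager's list, loads each Events entry as static data, then runs HandleFirstDay immediately or on a time-manager timer after InitialEventDelay.
; HandleFirstDay builds a BP_GE_DayResults from the custom title and description and queues it as a produced event.
; Init, Deinit and Unload are empty, and the work-day and day-change bindings are disconnected.
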(event `Init`
  (params (`Game Manager` :type "/Game/BP_Core/BP_Gamemode Object Reference")))

(event `Deinit`
  (params (`Game Manager` :type "/Game/BP_Core/BP_Gamemode Object Reference")))

(event `Handle First Day`
  (params (NewParam :type "/Game/BP_Core/TimeManagement/BP_Timer Object Reference"))
  (bind _ggameeventmanager (`/Game/BP_Core/BP_Gamemode.GGameEventManager` (`self.Game Manager`)))
  (bind _returnvalue (`|GenericCreateObject` "/Game/GameData/GameEvents/DayBeginEndEvents/BP_GE_DayResults.BP_GE_DayResults_C" self (`self.Custom Event Title`)))
  (`/Game/GameData/GameEvents/DayBeginEndEvents/BP_GE_DayResults.Make Description` _returnvalue (`self.Custom Event Description`))
  (`KismetArrayLibrary.Array_Add` (`/Game/BP_Core/GameEventManagement/BP_GameEventManager.Produced Events` _ggameeventmanager) _returnvalue)
  (`/Game/BP_Core/GameEventManagement/BP_GameEventManager.Produced Event Handler` _ggameeventmanager null))

(fn `Load`
  (params (`Game Manager` :type "/Game/BP_Core/BP_Gamemode Object Reference"))
  (bind _ggameeventmanager (`/Game/BP_Core/BP_Gamemode.GGameEventManager` `Game Manager`))
  (set `self.Game Manager` `Game Manager`)
  (`KismetArrayLibrary.Array_Clear` (`/Game/BP_Core/GameEventManagement/BP_GameEventManager.All Events` _ggameeventmanager))
  (for _array_element (`self.Events`)
    (set `/Game/BP_Core/GameEventManagement/BP_GameEventManager.Static Data` _array_element _ggameeventmanager)
    (`/Game/BP_Core/GameEventManagement/BP_GameEventManager.Load Static Data` _ggameeventmanager))
  (if (> (`/Game/BP_Core/TimeManagement/BP_TimeFuncs.Game Time to Minutes` (`self.Initial Event Delay`)) 0)
    (`/Game/BP_Core/TimeManagement/BP_TimeManager.Create Timer` (`/Game/BP_Core/BP_Gamemode.GTimeManager` `Game Manager`) (`self.Initial Event Delay`) (`|CreateDelegate` :!event `Handle First Day`))
    (else
      (`self.Handle First Day` null))))

(fn `Unload`
  (params (`Game Manager` :type "/Game/BP_Core/BP_Gamemode Object Reference")))