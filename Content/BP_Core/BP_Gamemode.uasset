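; Game mode that bootstraps the game's simulation managers and HUD on BeginPlay.
; SetupManagers spawns time, resource, profession, building, person, weather and game event manager actors, stores references to them, then calls CallGameInitialized.
; SetupUI then creates debug resource and weather widgets, the main HUD and an initially hidden person widget, connecting each to its manager.
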(event `self.ReceiveBeginPlay`
  (`self.SetupManagers`)
  (`self.SetupUI`))

(fn `SetupManagers`
  (bind _returnvalue (`self.GetTransform`))
  ;[1 1 1] Time Manager
  (bind _returnvalue_2 (`|SpawnActorFromClass` "/Game/BP_Core/TimeManagement/BP_TimeManager.BP_TimeManager_C" _returnvalue "AlwaysSpawn" "OverrideRootScale" null null))
  (set `self.GTimeManager` _returnvalue_2)
  (bind _returnvalue_3 (`|SpawnActorFromClass` "/Game/BP_Core/ResourceManagement/BP_UResourceManager.BP_UResourceManager_C" _returnvalue "AlwaysSpawn" "OverrideRootScale" null null))
  (set `self.GResourceManager` _returnvalue_3)
  (bind _returnvalue_4 (`|SpawnActorFromClass` "/Game/BP_Core/ProfessionManagement/BP_ProfessionManager.BP_ProfessionManager_C" _returnvalue "AlwaysSpawn" "OverrideRootScale" null null))
  (set `self.GProfessionsManager` _returnvalue_4)
  (bind _returnvalue_5 (`|SpawnActorFromClass` "/Game/BP_Core/BuildingManagement/BP_BuildingManager.BP_BuildingManager_C" _returnvalue "AlwaysSpawn" "OverrideRootScale" null null))
  (set `self.GBuildingManager` _returnvalue_5)
  (bind _returnvalue_6 (`|SpawnActorFromClass` "/Game/BP_Core/PeopleManagement/BP_PersonManager.BP_PersonManager_C" _returnvalue "AlwaysSpawn" "OverrideRootScale" null null))
  (set `self.GPersonManager` _returnvalue_6)
  (bind _returnvalue_7 (`|SpawnActorFromClass` "/Game/BP_Core/WeatherManagement/BP_WeatherManager.BP_WeatherManager_C" _returnvalue "AlwaysSpawn" "OverrideRootScale" null null))
  (set `self.GWeatherManager` _returnvalue_7)
  (bind _returnvalue_8 (`|SpawnActorFromClass` "/Game/BP_Core/GameEventManagement/BP_GameEventManager.BP_GameEventManager_C" _returnvalue "Undefined" "OverrideRootScale" null null))
  (set `self.GGameEventManager` _returnvalue_8)
  (`self.GameInitialized`)
  (return))

(fn `SetupUI`
  (bind _gresourcemanager (`self.GResourceManager`))
  (`|ExecutionSequence`
    (:`then_0`
      (bind _returnvalue (`|CreateWidget` "/Game/UI/BP/HUD_DBG_ResMan.HUD_DBG_ResMan_C"))
      (`UserWidget.AddToViewport` _returnvalue 0)
      (`/Game/UI/BP/HUD_DBG_ResMan.Connect to Managers` _returnvalue _gresourcemanager)
      (bind _values (`BlueprintMapLibrary.Map_Values` (`/Game/BP_Core/ResourceManagement/BP_UResourceManager.Resources` _gresourcemanager)))
      (`/Game/UI/BP/HUD_DBG_ResMan.Create Widgets` _returnvalue _values))
    (:`then_1`
      (bind _returnvalue_2 (`|CreateWidget` "/Game/UI/BP/WeatherWudget/DBG_HUD_Weather.DBG_HUD_Weather_C"))
      (`UserWidget.AddToViewport` _returnvalue_2 0)
      (`/Game/UI/BP/WeatherWudget/DBG_HUD_Weather.Init` _returnvalue_2 (`self.GWeatherManager`)))
    (:`then_2`
      (bind _returnvalue_3 (`|CreateWidget` "/Game/UI/Widgets/TimerAndScreenButtons/BP_HUD.BP_HUD_C"))
      (`UserWidget.AddToViewport` _returnvalue_3 0)
      (set `self.WTimer Widget` _returnvalue_3)
      (`/Game/UI/Widgets/TimerAndScreenButtons/BP_HUD.ConnectToManager` _returnvalue_3 (`self.GTimeManager`))
      (bind _returnvalue_4 (`|CreateWidget` "/Game/UI/Widgets/PersonWidgets/BP_PersonWidget.BP_PersonWidget_C"))
      (set `self.WPerson Widget` _returnvalue_4)
      (`UserWidget.AddToViewport` _returnvalue_4 0)
      (`Widget.SetVisibility` _returnvalue_4 "Hidden")
      (`/Game/UI/Widgets/PersonWidgets/BP_PersonWidget.ConnectToManager` _returnvalue_4 (`self.GPersonManager`)))))

(fn `UserConstructionScript`)