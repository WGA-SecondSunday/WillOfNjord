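; BP_GameEvent is a game event run under an EventManager, pairing a set of Conditions with selectable timed Actions.
; Init and Deinit pass setup and teardown on to every condition and action.
; CheckConditions succeeds only if all conditions pass.
; Activate enables the action at a given index, updates availability and activation count and returns that action's duration, while Deactivate disables it and makes the event available again.
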(event `Init`
  (params (`Event Manager` :type "/Game/BP_Core/GameEventManagement/BP_GameEventManager Object Reference"))
  (set `self.Event Manager` `Event Manager`)
  (for _array_element (`self.Conditions`)
    (`/Game/BP_Core/GameEventManagement/BP_GameEventCondition.Init` _array_element self))
  (for _array_element_2 (`self.Actions`)
    (`/Game/BP_Core/GameEventManagement/BP_GameEventAction.Init` (break `/Game/BP_Core/GameEventManagement/S_ActionAndDuration` _array_element_2) self)))

(event `Deinit`
  (for _array_element (`self.Conditions`)
    (`/Game/BP_Core/GameEventManagement/BP_GameEventCondition.Deinit` _array_element))
  (for _array_element_2 (`self.Actions`)
    (`/Game/BP_Core/GameEventManagement/BP_GameEventAction.Deinit` (break `/Game/BP_Core/GameEventManagement/S_ActionAndDuration` _array_element_2))))

(fn `Activate`
  (params (Action :type Integer))
  (returns (Duration :type "/Game/BP_Core/TimeManagement/BP_GameTime Structure"))
  (if (< Action (`KismetArrayLibrary.Array_Length` (`self.Actions`)))
    (bind _output_get (set `self.Chosen Action` Action))
    (set `self.Active` true)
    (set `self.Available` false)
    (`/Engine/EditorBlueprintResources/StandardMacros.IncrementInt` (`self.Number Of Activations`)
      (:`  `
        (bind (_output_action _output_duration) (break `/Game/BP_Core/GameEventManagement/S_ActionAndDuration` (`|GetArrayItem` (`self.Actions`) _output_get)))
        (`/Game/BP_Core/GameEventManagement/BP_GameEventAction.Enable` _output_action)
        (return _output_duration)))))

(fn `CheckConditions`
  (returns (Satisfied :type Boolean))
  (for _array_element (`self.Conditions`)
    (bind _result (`/Game/BP_Core/GameEventManagement/BP_GameEventCondition.CheckSelf` _array_element))
    (if (not _result)
      (return false)))
  (return true))

(fn `Deactivate`
  (bind _chosen_action (`self.Chosen Action`))
  (bind _output_action (break `/Game/BP_Core/GameEventManagement/S_ActionAndDuration` (`|GetArrayItem` (`self.Actions`) _chosen_action)))
  (if (>= _chosen_action 0)
    (set `self.Active` false)
    (set `self.Available` true)
    (`/Game/BP_Core/GameEventManagement/BP_GameEventAction.Disable` _output_action)
    (set `self.Chosen Action` -1)
    (return)))