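; Game event manager actor that schedules random and day-start events, shows them to the player and tracks active ones.
; It instantiates events from static data and, each new day, registers timers through the game's time manager; the day-end timer is unwired.
; Timed production randomly picks an event passing its conditions, and handlers pause the game to show an event widget.
; Selecting an action activates the event, with a timer for later deactivation.
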(event `self.ReceiveBeginPlay`
  (`parent.ReceiveBeginPlay`)
  (`self.Load Static Data`)
  (`|ExecutionSequence`
    (:`then_0`
      (add `/Game/BP_Core/TimeManagement/BP_TimeManager.OnDayChange` (`/Game/BP_Core/BP_Gamemode.GTimeManager` (`self.GameManager`)) (delegate `CustomEvent_0`)))
    (:`then_1`
      (`self.Register Self Timers` :!label _label))))

(event `CustomEvent_0`
  (params (`New Time` :type "/Game/BP_Core/TimeManagement/BP_GameTime Structure"))
  (goto _label))

(event `Event Selected`
  (params (`Event Idx` :type Integer) (`Action Idx` :type Integer))
  (bind _produced_events (`self.Produced Events`))
  (bind _active_events (`self.Active Events`))
  (bind _returnvalue (`KismetArrayLibrary.Array_Add` _active_events (`|GetArrayItem` _produced_events `Event Idx`)))
  (`KismetArrayLibrary.Array_Clear` _produced_events)
  (bind _output (`|GetArrayItem` _active_events _returnvalue))
  (bind _duration (`/Game/BP_Core/GameEventManagement/BP_GameEvent.Activate` _output `Action Idx`))
  (`self.OnEventActivated` _output)
  (`/Game/BP_Core/TimeManagement/BP_TimeManager.Create Timer` (`/Game/BP_Core/BP_Gamemode.GTimeManager` (`self.GameManager`)) _duration (delegate `Event Elapsed`)))

(event `Event Elapsed`
  (params (Timer :type "/Game/BP_Core/TimeManagement/BP_Timer Object Reference"))
  (bind _output (`|GetArrayItem` (`self.Active Events`) (stale `Event Selected` _returnvalue)))
  (`/Game/BP_Core/GameEventManagement/BP_GameEvent.Deactivate` _output)
  (`self.OnEventDeactivated` _output)
  (`KismetArrayLibrary.Array_RemoveItem` (`self.Active Events`) _output))

(fn `Handle Day Beggining`
  (params (Timer :type "/Game/BP_Core/TimeManagement/BP_Timer Object Reference"))
  (bind _returnvalue (`|GenericCreateObject` (`/Game/BP_Core/GameEventManagement/BPDA_GameEvents.Day Beginning Event` (`self.Static Data`)) self))
  (`/Game/BP_Core/GameEventManagement/BP_GameEvent.Init` _returnvalue self)
  (`KismetArrayLibrary.Array_Add` (`self.Produced Events`) _returnvalue)
  (`self.Produced Event Handler` null))

(fn `Handle Day Ending`
  (params (Timer :type "/Game/BP_Core/TimeManagement/BP_Timer Object Reference"))
  (bind _returnvalue (`|GenericCreateObject` (`/Game/BP_Core/GameEventManagement/BPDA_GameEvents.Day Ending Event` (`self.Static Data`)) self))
  (`/Game/BP_Core/GameEventManagement/BP_GameEvent.Init` _returnvalue self)
  (`KismetArrayLibrary.Array_Add` (`self.Produced Events`) _returnvalue)
  (`self.Produced Event Handler` null))

(fn `Handle Timer`
  (params (Timer :type "/Game/BP_Core/TimeManagement/BP_Timer Object Reference"))
  (`self.Produce New Events`)
  (return))

(fn `Load Static Data`
  (set `self.Event Times` (`/Game/BP_Core/GameEventManagement/BPDA_GameEvents.Event Times` (`self.Static Data`)))
  (for _array_element (`/Game/BP_Core/GameEventManagement/BPDA_GameEvents.Events` (`self.Static Data`))
    (bind _returnvalue (`|GenericCreateObject` _array_element self))
    (`/Game/BP_Core/GameEventManagement/BP_GameEvent.Init` _returnvalue self)
    (`KismetArrayLibrary.Array_Add` (`self.All Events`) _returnvalue)))

(fn `Produce New Events`
  (locals (`Available Events` :type "Array of /Game/BP_Core/GameEventManagement/BP_GameEvent Object Reference"))
  (bind _produced_events (`self.Produced Events`))
  (bind _available_events (`local.Available Events`))
  (bind _returnvalue (`KismetArrayLibrary.Array_Length` _available_events))
  (bind _output (`|GetArrayItem` _available_events (`KismetMathLibrary.RandomIntegerInRange` 0 (- _returnvalue 1))))
  (`KismetArrayLibrary.Array_Clear` _produced_events)
  (for _array_element (`self.All Events`)
    (bind _satisfied (`/Game/BP_Core/GameEventManagement/BP_GameEvent.CheckConditions` _array_element))
    (if _satisfied
      (`KismetArrayLibrary.Array_Add` (`local.Available Events`) _array_element)))
  (if (> _returnvalue 0)
    (`KismetArrayLibrary.Array_Add` _produced_events _output)
    (`self.OnEventsProduced` _output)))

(fn `Produced Event Handler`
  (params (NewParam :type "/Game/BP_Core/GameEventManagement/BP_GameEvent Object Reference"))
  (`GameplayStatics.SetGamePaused` true)
  (bind _returnvalue (`|CreateWidget` "/Game/UI/Widgets/EventWidget/EventWidget.EventWidget_C"))
  (`/Game/UI/Widgets/EventWidget/EventWidget.Init` _returnvalue (`|GetArrayItem` (`self.Produced Events`)))
  (`UserWidget.AddToViewport` _returnvalue 0))

(fn `Register Self Timers`
  (bind _gtimemanager (`/Game/BP_Core/BP_Gamemode.GTimeManager` (`self.GameManager`)))
  (`|ExecutionSequence`
    (:`then_0`
      (for _array_element (`self.Event Times`)
        (`/Game/BP_Core/TimeManagement/BP_TimeManager.Create Timer` _gtimemanager _array_element (`|CreateDelegate` :!event `Handle Timer`))))
    (:`then_1`
      (`/Game/BP_Core/TimeManagement/BP_TimeManager.Create Timer` _gtimemanager (`/Game/BP_Core/GameEventManagement/BPDA_GameEvents.Day Begin Event Time` (`self.Static Data`)) (`|CreateDelegate` :!event `Handle Day Beggining`)))))

(fn `UserConstructionScript`
  (`parent.UserConstructionScript`)
  (add `self.OnEventsProduced` (`|CreateDelegate` :!event `Produced Event Handler`)))