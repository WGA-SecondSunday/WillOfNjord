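; BP_GameEvent_Static provides a helper that builds a runtime BP_GameEvent object from GameEventInfo data.
; LoadGEventFromGEInfo constructs the event with the given Owner as outer, then copies its texts, duration and apply-once flag.
; It instantiates each action and condition class with the event as outer, adds them to the event's arrays and returns the event.
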(fn `Load GEvent From GEInfo`
  (params (Owner :type "Object Object Reference") (`Game Event Info` :type "/Game/BP_Core/GameEventManagement/BP_GameEvent_Info Structure"))
  (returns (`Game Event` :type "/Game/BP_Core/GameEventManagement/BP_GameEvent Object Reference"))
  (locals (Event :type "/Game/BP_Core/GameEventManagement/BP_GameEvent Object Reference"))
  (bind _returnvalue (`|GenericCreateObject` "/Game/BP_Core/GameEventManagement/BP_GameEvent.BP_GameEvent_C" Owner))
  (bind _output_get (set `local.Event` _returnvalue))
  (`|ExecutionSequence`
    (:`then_0`
      (set `/Game/BP_Core/GameEventManagement/BP_GameEvent.Texts` `Game Event Info_Texts_11_DAF4D6D942F231933711E58AE04BAF00` _output_get))
    (:`then_1`
      (set `/Game/BP_Core/GameEventManagement/BP_GameEvent.Duration` `Game Event Info_Duration_12_0BA69F9E437828C16002BEBB673C9DC2` _output_get))
    (:`then_2`
      (set `/Game/BP_Core/GameEventManagement/BP_GameEvent.Only Once` `Game Event Info_MayBeAppliedOnce_10_24E782C84669FB1FC73DB198CA6612C0` _output_get))
    (:`then_3`
      (for _array_element `Game Event Info_Actions_21_9BE765584DEEBC9BF9EF33BBFCAB312D`
        (bind _returnvalue_2 (`|GenericCreateObject` _array_element _output_get))
        (`KismetArrayLibrary.Array_Add` (`/Game/BP_Core/GameEventManagement/BP_GameEvent.Actions` _output_get) _returnvalue_2)))
    (:`then_4`
      (for _array_element_2 `Game Event Info_Conditions_20_99C16B8E428ED08152F40595EC33BA03`
        (bind _returnvalue_3 (`|GenericCreateObject` _array_element_2 _output_get))
        (`KismetArrayLibrary.Array_Add` (`/Game/BP_Core/GameEventManagement/BP_GameEvent.Conditions` _output_get) _returnvalue_3)))
    (:`then_5`
      (return (`local.Event`)))))