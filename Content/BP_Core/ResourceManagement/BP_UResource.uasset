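; BP_UResource is a data object for a single resource, holding its type, amount, goal and count of times the goal was reached.
; Initialize sets all four fields and GetAll returns them together.
; UpdateAmount overwrites the amount and fires OnAmountChanged.
; It then increments the count and fires OnGoalReached when Amount modulo Goal is at least that count, a remainder test rather than a count of whole goals.
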(fn `GetAll`
  (returns (`Resource Type` :type "/Game/BP_Core/ResourceManagement/BP_ResourceTypes Enum") (Amount :type "Float (double-precision)") (Goal :type "Float (double-precision)") (`Goal Reached Times` :type Integer))
  (return (`self.Resource Type`) (`self.Amount`) (`self.Goal`) (`self.Goal Reached Times`)))

(fn `Initialize`
  (params (`Resource Type` :type "/Game/BP_Core/ResourceManagement/BP_ResourceTypes Enum" :default "NewEnumerator5") (Amount :type "Float (double-precision)") (Goal :type "Float (double-precision)") (`Goal Reached Times` :type Integer))
  (set `self.Resource Type` `Resource Type`)
  (set `self.Amount` Amount)
  (set `self.Goal` Goal)
  (set `self.Goal Reached Times` `Goal Reached Times`)
  (return))

(fn `UpdateAmount`
  (params (`New Amount` :type "Float (double-precision)"))
  (bind _goal_reached_times (`self.Goal Reached Times`))
  (bind _output_get (set `self.Amount` `New Amount`))
  (`self.OnAmountChanged` self)
  (if (>= (mod _output_get (`self.Goal`)) (`KismetMathLibrary.Conv_IntToDouble` _goal_reached_times))
    (`/Engine/EditorBlueprintResources/StandardMacros.IncrementInt` _goal_reached_times
      (:`  `
        (`self.OnGoalReached` self))))
  (return))