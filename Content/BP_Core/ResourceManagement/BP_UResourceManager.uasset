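; Resource manager that owns the game's BP_UResource objects and sets their daily goals.
; Construction builds a map of visible resources per type plus hidden special resources with fixed settings.
; On day change, it resets auto-drop resources and recalculates visible goals from counts of people in high, medium and low efficiency tiers.
; The weather multiplier setter only stores its value; its goal-scaling loop is disconnected.
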(event `self.ReceiveBeginPlay`
  (`parent.ReceiveBeginPlay`)
  (add `/Game/BP_Core/BP_Gamemode.GameInitialized` (`self.GameManager`) (delegate `CustomEvent_0`)))

(event `CustomEvent_0`
  (add `/Game/BP_Core/TimeManagement/BP_TimeManager.OnDayChange` (`/Game/BP_Core/BP_Gamemode.GTimeManager` (`self.GameManager`)) (`|CreateDelegate` :!event `Handle Day Change`)))

(fn `Handle Day Change`
  (params (Time :type "/Game/BP_Core/TimeManagement/BP_GameTime Structure"))
  (locals (`High Count` :type Integer) (`Med Count` :type Integer) (`Low Count` :type Integer))
  (bind _max_amount_per_day (`self.Max Amount Per Day`))
  (`|ExecutionSequence`
    (:`then_0`
      (for _array_element (`/Game/BP_Core/PeopleManagement/BP_PersonManager.People` (`/Game/BP_Core/BP_Gamemode.GPersonManager` (`self.GameManager`)))
        (bind _tag (`/Game/BP_Core/PeopleManagement/BP_Person.Get Efficiency Tag` _array_element))
        (switch `int` _tag
          (:`0`
            (`/Engine/EditorBlueprintResources/StandardMacros.IncrementInt` (`local.High Count`)))
          (:`1`
            (`/Engine/EditorBlueprintResources/StandardMacros.IncrementInt` (`local.Med Count`)))
          (:`2`
            (`/Engine/EditorBlueprintResources/StandardMacros.IncrementInt` (`local.Low Count`))))))
    (:`then_1`
      (bind _values (`BlueprintMapLibrary.Map_Values` (`self.Resources`)))
      (for _array_element_2 _values
        (if (`/Game/BP_Core/ResourceManagement/BP_UResource.Auto Drop` _array_element_2)
          (set `/Game/BP_Core/ResourceManagement/BP_UResource.Goal Reached Times` 0 _array_element_2)
          (`/Game/BP_Core/ResourceManagement/BP_UResource.UpdateAmount` _array_element_2 0.0))
        (if (not (`/Game/BP_Core/ResourceManagement/BP_UResource.Hidden` _array_element_2))
          (`/Game/BP_Core/ResourceManagement/BP_UResource.Update Goal` _array_element_2 (+ (* _max_amount_per_day (* (`local.High Count`) (`self.High Factor`))) (* _max_amount_per_day (* (`local.Med Count`) (`self.Med Factor`))) (* _max_amount_per_day (* (`local.Low Count`) (`self.Low Factor`)))))))
      (return))))

(fn `Set New Day Goal Multiplier`
  (params (`Global Multiplier` :type "Float (double-precision)"))
  (set `self.Weather Multiplier` `Global Multiplier`))

(fn `UserConstructionScript`
  (bind _resources (`self.Resources`))
  (`parent.UserConstructionScript`)
  (`|ExecutionSequence`
    (:`then_0`
      (bind _enumvalue (foreach `/Game/BP_Core/ResourceManagement/BP_ResourceTypes` false)
        (:`LoopBody`
          (bind _returnvalue (`|GenericCreateObject` "/Game/BP_Core/ResourceManagement/BP_UResource.BP_UResource_C" self))
          (`/Game/BP_Core/ResourceManagement/BP_UResource.Initialize` _returnvalue _enumvalue 0.0 (`self.Current Day Base Goal`) 0)
          (`BlueprintMapLibrary.Map_Add` _resources _enumvalue _returnvalue))))
    (:`then_1`
      (bind _returnvalue_2 (`|GenericCreateObject` "/Game/BP_Core/ResourceManagement/BP_UResource.BP_UResource_C" self false))
      (`/Game/BP_Core/ResourceManagement/BP_UResource.Initialize` _returnvalue_2 "NewEnumerator6" 0.0 0.0 0)
      (set `/Game/BP_Core/ResourceManagement/BP_UResource.Hidden` true _returnvalue_2)
      (`BlueprintMapLibrary.Map_Add` _resources "NewEnumerator6" _returnvalue_2))
    (:`then_2`
      (bind _returnvalue_3 (`|GenericCreateObject` "/Game/BP_Core/ResourceManagement/BP_UResource.BP_UResource_C" self false))
      (`/Game/BP_Core/ResourceManagement/BP_UResource.Initialize` _returnvalue_3 "NewEnumerator7" 6.0 100000.0 0)
      (set `/Game/BP_Core/ResourceManagement/BP_UResource.Hidden` true _returnvalue_3)
      (`BlueprintMapLibrary.Map_Add` _resources "NewEnumerator7" _returnvalue_3))
    (:`then_3`
      (bind _returnvalue_4 (`|GenericCreateObject` "/Game/BP_Core/ResourceManagement/BP_UResource.BP_UResource_C" self false))
      (`/Game/BP_Core/ResourceManagement/BP_UResource.Initialize` _returnvalue_4 "NewEnumerator8" 0.0 5000.0 0)
      (set `/Game/BP_Core/ResourceManagement/BP_UResource.Hidden` true _returnvalue_4)
      (`BlueprintMapLibrary.Map_Add` _resources "NewEnumerator8" _returnvalue_4))
    (:`then_4`
      (bind _returnvalue_5 (`|GenericCreateObject` "/Game/BP_Core/ResourceManagement/BP_UResource.BP_UResource_C" self true))
      (`/Game/BP_Core/ResourceManagement/BP_UResource.Initialize` _returnvalue_5 "NewEnumerator9" 0.0 1000000.0 0)
      (set `/Game/BP_Core/ResourceManagement/BP_UResource.Hidden` true _returnvalue_5)
      (`BlueprintMapLibrary.Map_Add` _resources "NewEnumerator9" _returnvalue_5))
    (:`then_5`
      (bind _returnvalue_6 (`|GenericCreateObject` "/Game/BP_Core/ResourceManagement/BP_UResource.BP_UResource_C" self))
      (`/Game/BP_Core/ResourceManagement/BP_UResource.Initialize` _returnvalue_6 "NewEnumerator10" 0.0 100.0 0)
      (set `/Game/BP_Core/ResourceManagement/BP_UResource.Hidden` true _returnvalue_6)
      (`BlueprintMapLibrary.Map_Add` _resources "NewEnumerator10" _returnvalue_6))))