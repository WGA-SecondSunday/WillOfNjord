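; BP_ResourceManager holds the game's list of resources, each with an amount, daily goal and goal-reached count.
; The construction script seeds one entry per resource type, and BeginPlay binds to the time manager's hour-change event.
; UpdateResources adds a random amount to every resource as a testing placeholder, then broadcasts the array through OnAllResourceUpdate.
; BroadcastResourceUpdates is an empty stub.
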(event `self.ReceiveBeginPlay`
  (`parent.ReceiveBeginPlay`)
  (add `/Game/BP_Core/TimeManagement/BP_TimeManager.OnHourChange` (`/Game/BP_Core/BP_Gamemode.GTimeManager` (`self.GameManager`)) (`|CreateDelegate` :!event `Update Resources`)))

(fn `BroadcastResourceUpdates`)

(fn `Update Resources`
  (params (`New Time` :type "/Game/BP_Core/TimeManagement/BP_GameTime Structure"))
  (bind _resources (`self.Resources`))
  (for (_array_element _array_index) _resources
    (bind (_resourcetype _amount _dailygoal _goalreachedtimes) (break `/Game/BP_Core/ResourceManagement/BP_Resource` _array_element))
    (`KismetArrayLibrary.Array_Set` _resources _array_index (make `/Game/BP_Core/ResourceManagement/BP_Resource` _resourcetype (+ _amount (`KismetMathLibrary.RandomFloatInRange` 2.0 20.0)) _dailygoal _goalreachedtimes)))
  (`self.OnAllResourceUpdate` _resources)
  (return))

(fn `UserConstructionScript`
  (bind _enumvalue (foreach `/Game/BP_Core/ResourceManagement/BP_ResourceTypes` false)
    (:`LoopBody`
      (`KismetArrayLibrary.Array_Add` (`self.Resources`) (make `/Game/BP_Core/ResourceManagement/BP_Resource` _enumvalue)))))