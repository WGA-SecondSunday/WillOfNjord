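; Weather manager that sets a new weather state on day change and turns it into global gameplay modifiers.
; It binds to the time manager's day change, then generates, stores, applies and broadcasts the weather.
; Visibility drives profession efficiency, temperature updates resource goals, and wind scales building speed, each as neutral, buff or debuff.
; Generation is currently hardcoded to return buff for all three.
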(event `self.ReceiveBeginPlay`
  (`parent.ReceiveBeginPlay`)
  (add `/Game/BP_Core/TimeManagement/BP_TimeManager.OnDayChange` (`/Game/BP_Core/BP_Gamemode.GTimeManager` (`self.GameManager`)) (`|CreateDelegate` :!event `DayChangedHandler`)))

(fn `ApplyWeather`
  (params (Weather :type "/Game/BP_Core/WeatherManagement/BP_Weather Structure"))
  (bind _gamemanager (`self.GameManager`))
  (bind _gprofessionsmanager (`/Game/BP_Core/BP_Gamemode.GProfessionsManager` _gamemanager))
  (bind _gresourcemanager (`/Game/BP_Core/BP_Gamemode.GResourceManager` _gamemanager))
  (bind _gbuildingmanager (`/Game/BP_Core/BP_Gamemode.GBuildingManager` _gamemanager))
  (`|ExecutionSequence`
    (:`then_0`
      (switch `/Game/BP_Core/WeatherManagement/BP_WeatherValues` Weather_Visibility_4_F54C7CF64130344356123B80971921CF
        (:`NewEnumerator0`
          (set `/Game/BP_Core/ProfessionManagement/BP_ProfessionManager.Global Efficiency` 1.0 _gprofessionsmanager))
        (:`NewEnumerator1`
          (set `/Game/BP_Core/ProfessionManagement/BP_ProfessionManager.Global Efficiency` (`self.Visibility_BuffEfficiency`) _gprofessionsmanager))
        (:`NewEnumerator2`
          (set `/Game/BP_Core/ProfessionManagement/BP_ProfessionManager.Global Efficiency` (`self.Visibility_DebuffEficciency`) _gprofessionsmanager))))
    (:`then_1`
      (switch `/Game/BP_Core/WeatherManagement/BP_WeatherValues` Weather_Temperature_5_CE45D8E0414ACB2A079E09AFB61A05AF
        (:`NewEnumerator0`
          (`/Game/BP_Core/ResourceManagement/BP_UResourceManager.Update Goal For All` _gresourcemanager 1.0))
        (:`NewEnumerator1`
          (`/Game/BP_Core/ResourceManagement/BP_UResourceManager.Update Goal For All` _gresourcemanager (`self.Temperature_BuffEfficiency`)))
        (:`NewEnumerator2`
          (`/Game/BP_Core/ResourceManagement/BP_UResourceManager.Update Goal For All` _gresourcemanager (`self.Temperature_DebuffEfficiency`)))))
    (:`then_2`
      (switch `/Game/BP_Core/WeatherManagement/BP_WeatherValues` Weather_Wind_6_12C841664C00600E69DB89A472311C04
        (:`NewEnumerator0`
          (set `/Game/BP_Core/BuildingManagement/BP_BuildingManager.Global Building Speed Factor` 1.0 _gbuildingmanager))
        (:`NewEnumerator1`
          (set `/Game/BP_Core/BuildingManagement/BP_BuildingManager.Global Building Speed Factor` (`self.Wind_BuffEfficiency`) _gbuildingmanager))
        (:`NewEnumerator2`
          (set `/Game/BP_Core/BuildingManagement/BP_BuildingManager.Global Building Speed Factor` (`self.Wind_DebuffEfficiency`) _gbuildingmanager))))))

(fn `DayChangedHandler`
  (params (`New Time` :type "/Game/BP_Core/TimeManagement/BP_GameTime Structure"))
  (bind _new_weather (`self.GenerateWeather`))
  (bind _output_get (set `self.CurrentWeather` _new_weather))
  (`self.ApplyWeather` _output_get)
  (`self.OnWeatherChanged` _output_get)
  (return))

(fn `GenerateWeather`
  (returns (`New Weather` :type "/Game/BP_Core/WeatherManagement/BP_Weather Structure"))
  (return (make `/Game/BP_Core/WeatherManagement/BP_Weather` "NewEnumerator1" "NewEnumerator1" "NewEnumerator1")))

(fn `UserConstructionScript`
  (`parent.UserConstructionScript`))