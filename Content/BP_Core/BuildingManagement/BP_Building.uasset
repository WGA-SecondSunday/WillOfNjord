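; Building actor that is constructed, upgraded and demolished through a manager's queue, boosting one profession's worker capacity and efficiency per level.
; Status parity encodes the phase: odd is under construction with meshes hidden behind a status widget, even is a finished level.
; Status changes cancel or apply that level's effect.
; Upgrades consume a resource; demolition refunds cost and frees the spawn spot; left-click toggles an info widget.
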(event `self.ReceiveActorOnClicked`
  (params (ButtonPressed :type "Key Structure"))
  (bind _bp_3dplayerfacingwidget (`self.BP_3DPlayerFacingWidget`))
  (if (== ButtonPressed "LeftMouseButton")
    (`/Engine/EditorBlueprintResources/StandardMacros.FlipFlop`
      (:`A`
        (`SceneComponent.SetVisibility` _bp_3dplayerfacingwidget true true)
        (`/Game/UI/Widgets/BuildingInfoWidgets/BP_3DPlayerFacingWidget.Set Widget` _bp_3dplayerfacingwidget "/Game/UI/Widgets/BuildingInfoWidgets/BP_BuildingInfoW.BP_BuildingInfoW_C"))
      (:`B`
        (`SceneComponent.SetVisibility` _bp_3dplayerfacingwidget false true)))))

(event `Init`
  (params (BuildMan :type "/Game/BP_Core/BuildingManagement/BP_BuildingManager Object Reference"))
  (set `self.Buildings Manager` BuildMan)
  (add `self.OnStatusChanged` (`|CreateDelegate` :!event `Status Changed Handler`))
  (add `self.OnDestroyed` (`|CreateDelegate` :!event `Event Destroyed`))
  (`self.Trigger Status Update` (`self.Constructing Time`)))

(event `Event Destroyed` :!signature `self.OnDestroyed`
  (params (DestroyedActor :type "Actor Object Reference"))
  (bind _asbp_spawn_spot (cast `/Game/BP_Core/BuildingManagement/BP_SpawnSpot` (`self.GetAttachParentActor`)))
  (set `/Game/BP_Core/BuildingManagement/BP_SpawnSpot.Empty` true _asbp_spawn_spot))

(event `self.ReceiveTick`
  (params (DeltaSeconds :type "Float (single-precision)")))

(fn `Apply Effect`
  (params (`New Level` :type Integer))
  (bind _value (`BlueprintMapLibrary.Map_Find` (`/Game/BP_Core/ProfessionManagement/BP_ProfessionManager.Professions` (`/Game/BP_Core/BP_Gamemode.GProfessionsManager` (`/Game/BP_Core/Base/BaseManager.GameManager` (`self.Buildings Manager`)))) (`self.Affected Profession`)))
  (`KismetArrayLibrary.Array_Add` (`/Game/BP_Core/ProfessionManagement/BP_Profession.Global Efficiencies` _value) (make `/Game/BP_Core/ProfessionManagement/BP_EfficiencyModifier` self (`|GetArrayItem` (`self.Efficiencies`) `New Level`)))
  (set `/Game/BP_Core/ProfessionManagement/BP_Profession.MaxWorkers` (+ (`/Game/BP_Core/ProfessionManagement/BP_Profession.MaxWorkers` _value) (`|GetArrayItem` (`self.Capacities`) `New Level`)) _value))

(fn `CancelEffect`
  (params (PrevLevel :type Integer))
  (locals (`To Delete` :type "Array of Integer"))
  (bind _value (`BlueprintMapLibrary.Map_Find` (`/Game/BP_Core/ProfessionManagement/BP_ProfessionManager.Professions` (`/Game/BP_Core/BP_Gamemode.GProfessionsManager` (`/Game/BP_Core/Base/BaseManager.GameManager` (`self.Buildings Manager`)))) (`self.Affected Profession`)))
  (bind _global_efficiencies (`/Game/BP_Core/ProfessionManagement/BP_Profession.Global Efficiencies` _value))
  (bind (_arrayindex _arrayelement) (`/Engine/EditorBlueprintResources/StandardMacros.ReverseForEachLoop` _global_efficiencies)
    (:`LoopBody`
      (if (== self (break `/Game/BP_Core/ProfessionManagement/BP_EfficiencyModifier` _arrayelement))
        (`KismetArrayLibrary.Array_Remove` _global_efficiencies _arrayindex)))
    (:`Completed`
      (set `/Game/BP_Core/ProfessionManagement/BP_Profession.MaxWorkers` (- (`/Game/BP_Core/ProfessionManagement/BP_Profession.MaxWorkers` _value) (`|GetArrayItem` (`self.Capacities`) PrevLevel)) _value))))

(fn `Check Conditions and Consume Cost`
  (returns (Success :type Boolean))
  (bind _buildings_manager (`self.Buildings Manager`))
  (bind _value (`BlueprintMapLibrary.Map_Find` (`/Game/BP_Core/ResourceManagement/BP_UResourceManager.Resources` (`/Game/BP_Core/BP_Gamemode.GResourceManager` (`/Game/BP_Core/Base/BaseManager.GameManager` _buildings_manager))) "NewEnumerator7"))
  (bind (_cost _satisfied) (`/Game/BP_Core/BuildingManagement/BP_BuildingManager.Check Cost` _buildings_manager (`GameplayStatics.GetObjectClass` self)))
  (if _satisfied
    (`/Game/BP_Core/ResourceManagement/BP_UResource.UpdateAmount` _value (- (`/Game/BP_Core/ResourceManagement/BP_UResource.Amount` _value) _cost))
    (return true)
    (else
      (return false))))

(fn `Check Level Condition`
  (params (Level :type Integer))
  (returns (Result :type Boolean))
  (return (< Level (`KismetMathLibrary.Min` (`KismetArrayLibrary.Array_Length` (`self.Efficiencies`)) (`KismetArrayLibrary.Array_Length` (`self.Capacities`))))))

(fn `EndStatusUpdate`
  (locals (`Old Status` :type Integer))
  (bind _buildings_manager (`self.Buildings Manager`))
  (bind _status (`self.Status`))
  (bind _value (`BlueprintMapLibrary.Map_Find` (`/Game/BP_Core/ResourceManagement/BP_UResourceManager.Resources` (`/Game/BP_Core/BP_Gamemode.GResourceManager` (`/Game/BP_Core/Base/BaseManager.GameManager` _buildings_manager))) "NewEnumerator7"))
  ;[1 1 1] Здание должно быть разрушено?
  (if (== _status 0)
    (`self.K2_DestroyActor`)
    (`/Game/BP_Core/ResourceManagement/BP_UResource.UpdateAmount` _value (+ (`/Game/BP_Core/ResourceManagement/BP_UResource.Amount` _value) (`BlueprintMapLibrary.Map_Find` (`/Game/BP_Core/BuildingManagement/BP_BuildingManager.Building Costs` _buildings_manager) (`GameplayStatics.GetObjectClass` self))))
    (`KismetArrayLibrary.Array_RemoveItem` (`/Game/BP_Core/BuildingManagement/BP_BuildingManager.Buildings` (`self.Buildings Manager`)) self)
    (else
      (set `local.Old Status` _status)
      (bind _result (`/Engine/EditorBlueprintResources/StandardMacros.IncrementInt` _status)
        (:`  `
          (`self.Set Building Mesh`)
          (`self.OnStatusChanged` self (`local.Old Status`) _result)))))
  (return))

(fn `Set Building Mesh`
  (`SceneComponent.SetVisibility` (`self.BP_3DPlayerFacingWidget`) false true)
  (for _array_element (`self.K2_GetComponentsByClass` "/Script/Engine.StaticMeshComponent")
    (`SceneComponent.SetVisibility` _array_element true true)))

(fn `Set Constructing Mesh`
  (bind _bp_3dplayerfacingwidget (`self.BP_3DPlayerFacingWidget`))
  (`SceneComponent.SetVisibility` _bp_3dplayerfacingwidget true true)
  (`/Game/UI/Widgets/BuildingInfoWidgets/BP_3DPlayerFacingWidget.Set Widget` _bp_3dplayerfacingwidget "/Game/UI/Widgets/BuildingInfoWidgets/BP_StatusChangeW.BP_StatusChangeW_C")
  (for _array_element (`self.K2_GetComponentsByClass` "/Script/Engine.StaticMeshComponent")
    (`SceneComponent.SetVisibility` _array_element false true)))

(fn `Status Changed Handler`
  (params (NewParam :type "/Game/BP_Core/BuildingManagement/BP_Building Object Reference") (`Old Status` :type Integer) (`New Status` :type Integer))
  (bind _returnvalue (- (/ `Old Status` 2) 1))
  (bind _returnvalue_2 (- (/ `New Status` 2) 1))
  (if (== (mod `Old Status` 2) 0)
    (if (>= _returnvalue 0)
      (`self.CancelEffect` _returnvalue))
    (elif (>= _returnvalue_2 0)
      (`self.Apply Effect` _returnvalue_2))))

(fn `Trigger Status Update`
  (params (`Status Change Duration` :type "/Game/BP_Core/TimeManagement/BP_GameTime Structure") (`Destroy Building` :type Boolean))
  (locals (`Old Status` :type Integer))
  (`self.Check Level Condition` (+ (/ (`self.Status`) 2) 1))
  (set `local.Old Status` (`self.Status`))
  (if `Destroy Building`
    (set `self.Status` 0)
    (`self.Set Constructing Mesh` :!label _label)
    (set `self.Status Change Time` `Status Change Duration`)
    (`/Game/BP_Core/BuildingManagement/BP_BuildingManager.Add To Building Queue` (`self.Buildings Manager`) self)
    (`self.OnStatusChanged` self (`local.Old Status`) (`self.Status`))
    (return)
    (else
      (bind _success (`self.Check Conditions and Consume Cost`))
      (if _success
        (`/Engine/EditorBlueprintResources/StandardMacros.IncrementInt` (`self.Status`)
          (:`  `
            (goto _label)))))))

(fn `UserConstructionScript`)