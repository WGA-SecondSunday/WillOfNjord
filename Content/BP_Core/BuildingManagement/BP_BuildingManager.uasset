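; Building manager that spawns and tracks buildings, loading per-class build conditions and costs from static data on BeginPlay.
; Spawning checks the class's condition unless bypassed, then attaches the building to its spot, initializes it and binds to its status changes.
; A proxy rebroadcasts status changes through the manager's own dispatcher.
; It also queues building tasks with a notification and compares costs against one resource in the GameManager's resource manager.
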(event `self.ReceiveBeginPlay`
  (`parent.ReceiveBeginPlay`)
  (`self.LoadStaticData`))

(fn `Add To Building Queue`
  (params (Building :type "/Game/BP_Core/BuildingManagement/BP_Building Object Reference"))
  (locals (`Need Event` :type Boolean))
  (bind _building_queue (`self.Building Queue`))
  (`KismetArrayLibrary.Array_Add` _building_queue Building)
  (if (> (`KismetArrayLibrary.Array_Length` _building_queue) 0)
    (`self.OnNewBuildingTask`)))

(fn `Building Status Proxy`
  (params (NewParam :type "/Game/BP_Core/BuildingManagement/BP_Building Object Reference") (NewParam1 :type Integer) (NewParam2 :type Integer))
  (`self.OnBuildingStatusChanged` NewParam NewParam1 NewParam2))

(fn `Check Cost`
  (params (Building :type "/Game/BP_Core/BuildingManagement/BP_Building Class Reference"))
  (returns (Cost :type "Float (double-precision)") (Satisfied :type Boolean))
  (bind _value (`BlueprintMapLibrary.Map_Find` (`self.Building Costs`) Building))
  (return _value (<= _value (`/Game/BP_Core/ResourceManagement/BP_UResource.Amount` (`BlueprintMapLibrary.Map_Find` (`/Game/BP_Core/ResourceManagement/BP_UResourceManager.Resources` (`/Game/BP_Core/BP_Gamemode.GResourceManager` (`self.GameManager`))) "NewEnumerator7")))))

(fn `LoadStaticData`
  (bind _staticdata (`self.StaticData`))
  (bind _output_get (set `self.Building Conditions` (`/Game/BP_Core/BuildingManagement/BPDA_BuildMan_BaseData.GetBuildingConditions` _staticdata)))
  (bind _values (`BlueprintMapLibrary.Map_Values` _output_get))
  (for _array_element _values
    (`/Game/BP_Core/BuildingManagement/BP_BuildingCondition.Init` _array_element self))
  (set `self.Building Costs` (`/Game/BP_Core/BuildingManagement/BPDA_BuildMan_BaseData.Costs` _staticdata)))

(fn `SpawnBuildingAtSpot`
  (params (Building :type "/Game/BP_Core/BuildingManagement/BP_Building Class Reference") (Spot :type "/Game/BP_Core/BuildingManagement/BP_SpawnSpot Object Reference"))
  (bind (_returnvalue_location _returnvalue_rotation) (`KismetMathLibrary.BreakTransform` (`self.GetTransform` Spot)))
  (bind (_value _returnvalue) (`BlueprintMapLibrary.Map_Find` (`self.Building Conditions`) Building))
  (if (`self.Condition Bypass`)
    (bind _returnvalue_2 (`|SpawnActorFromClass` Building (`KismetMathLibrary.MakeTransform` _returnvalue_location _returnvalue_rotation) "Undefined" "OverrideRootScale" null null :!label _label))
    (`self.K2_AttachToActor` _returnvalue_2 Spot "None" "KeepWorld" "KeepWorld" "KeepWorld" false)
    (`/Game/BP_Core/BuildingManagement/BP_Building.Init` _returnvalue_2 self)
    (add `/Game/BP_Core/BuildingManagement/BP_Building.OnStatusChanged` _returnvalue_2 (`|CreateDelegate` :!event `Building Status Proxy`))
    (`KismetArrayLibrary.Array_Add` (`self.Buildings`) _returnvalue_2)
    (return)
    (elif _returnvalue
      (bind _result (`/Game/BP_Core/BuildingManagement/BP_BuildingCondition.CheckCondition` _value self))
      (if _result
        (goto _label))
      (else
        (goto _label)))))

(fn `UserConstructionScript`
  (`parent.UserConstructionScript`))