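; BP_TimerFunctions provides GameTimeDecrease, which steps a Day/Hour/Minute countdown back ten in-game minutes per call.
; It returns true if the time is already all zero; otherwise it writes the decreased value back by reference and returns false.
; Borrowing triggers on reaching zero, resetting minutes to 60 and hours to 24, without clamping Day, so decrements skip the all-zero state.
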(fn `GameTime Decrease`
  (params (Time :type "/Game/BP_Core/TimeManagement/BP_GameTime Structure (by ref)"))
  (returns (`Timer Is Over` :type Boolean))
  (locals (Timer :type "/Game/BP_Core/TimeManagement/BP_GameTime Structure"))
  (bind _output_get (set `local.Timer` Time))
  ;[1 1 1] Время вышло?
  (if (and (== (break `/Game/BP_Core/TimeManagement/BP_GameTime` _output_get) 0) (== (`.Hour_7_F85BF52C4A7085BDBE2839A014EE0E99` (break `/Game/BP_Core/TimeManagement/BP_GameTime` _output_get)) 0) (== (`.Minute_8_834EBD4B490534C3A6916281989DF1A0` (break `/Game/BP_Core/TimeManagement/BP_GameTime` _output_get)) 0))
    (return true)
    (else
      ;[1 1 1] Уменьшение счетчика игрового времени
      (bind _output_get_2 (set `local.Timer` (make `/Game/BP_Core/TimeManagement/BP_GameTime` (break `/Game/BP_Core/TimeManagement/BP_GameTime` _output_get) (`.Hour_7_F85BF52C4A7085BDBE2839A014EE0E99` (break `/Game/BP_Core/TimeManagement/BP_GameTime` _output_get)) (- (`.Minute_8_834EBD4B490534C3A6916281989DF1A0` (break `/Game/BP_Core/TimeManagement/BP_GameTime` _output_get)) 10))))
      (if (== (`.Minute_8_834EBD4B490534C3A6916281989DF1A0` (break `/Game/BP_Core/TimeManagement/BP_GameTime` _output_get_2)) 0)
        (bind _output_get_3 (set `local.Timer` (make `/Game/BP_Core/TimeManagement/BP_GameTime` (break `/Game/BP_Core/TimeManagement/BP_GameTime` _output_get_2) (- (`.Hour_7_F85BF52C4A7085BDBE2839A014EE0E99` (break `/Game/BP_Core/TimeManagement/BP_GameTime` _output_get_2)) 1) 60)))
        (if (== (`.Hour_7_F85BF52C4A7085BDBE2839A014EE0E99` (break `/Game/BP_Core/TimeManagement/BP_GameTime` _output_get_3)) 0)
          (set `local.Timer` (make `/Game/BP_Core/TimeManagement/BP_GameTime` (- (break `/Game/BP_Core/TimeManagement/BP_GameTime` _output_get_3) 1) 24 (`.Minute_8_834EBD4B490534C3A6916281989DF1A0` (break `/Game/BP_Core/TimeManagement/BP_GameTime` _output_get_3))))))
      (`|VariableSetRef` Time (`local.Timer`))
      (return false))))