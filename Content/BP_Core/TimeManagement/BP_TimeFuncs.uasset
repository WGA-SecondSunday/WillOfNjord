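; BP_TimeFuncs is a function library for game time values made of day, hour and minute.
; Delta and division convert times to total minutes, do the math, then rebuild a time from the result.
; Delta is absolute, using max minus min.
; The conversions are asymmetric: to minutes uses 24-hour days, while from minutes splits hours into days by 60.
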(fn `Game Time Delta`
  (params (T1 :type "/Game/BP_Core/TimeManagement/BP_GameTime Structure") (T2 :type "/Game/BP_Core/TimeManagement/BP_GameTime Structure"))
  (returns (T :type "/Game/BP_Core/TimeManagement/BP_GameTime Structure"))
  (bind _minutes (`self.Game Time to Minutes` T1))
  (bind _minutes_2 (`self.Game Time to Minutes` T2))
  (return (`self.Game Time From Minutes` (- (`KismetMathLibrary.Max` _minutes _minutes_2) (`KismetMathLibrary.Min` _minutes _minutes_2)))))

(fn `Game Time Div`
  (params (Time :type "/Game/BP_Core/TimeManagement/BP_GameTime Structure") (Divisor :type Integer))
  (returns (Result :type "/Game/BP_Core/TimeManagement/BP_GameTime Structure"))
  (return (`self.Game Time From Minutes` (/ (`self.Game Time to Minutes` Time) Divisor))))

(fn `Game Time From Minutes`
  (params (Minutes :type Integer))
  (returns (Time :type "/Game/BP_Core/TimeManagement/BP_GameTime Structure"))
  (bind _returnvalue (/ Minutes 60))
  (return (make `/Game/BP_Core/TimeManagement/BP_GameTime` (/ _returnvalue 60) (mod _returnvalue 60) (mod Minutes 60))))

(fn `Game Time to Minutes`
  (params (Time :type "/Game/BP_Core/TimeManagement/BP_GameTime Structure"))
  (returns (Minutes :type Integer))
  (return (+ (* (+ (* Time_Day_6_A866B7A54F6E2E7BD5ACC7B9F2B0AFDD 24) Time_Hour_7_F85BF52C4A7085BDBE2839A014EE0E99) 60) Time_Minute_8_834EBD4B490534C3A6916281989DF1A0)))