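; BP_Timer is a countdown timer from the time management system that works on a day, hour and minute duration.
; Init flattens the given duration into total minutes.
; Each Tick call subtracts a fixed ten minutes, ignoring its Time input, and fires OnTimerEnd with itself when the count equals exactly zero.
; Durations that are not positive multiples of ten minutes therefore never fire the event.
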(event `Init`
  (params (Duration :type "/Game/BP_Core/TimeManagement/BP_GameTime Structure"))
  (set `self.Minutes Duration` (+ (* (+ (* Duration_Day_6_A866B7A54F6E2E7BD5ACC7B9F2B0AFDD 24) Duration_Hour_7_F85BF52C4A7085BDBE2839A014EE0E99) 60) Duration_Minute_8_834EBD4B490534C3A6916281989DF1A0)))

(fn `Tick`
  (params (Time :type "/Game/BP_Core/TimeManagement/BP_GameTime Structure"))
  (bind _output_get (set `self.Minutes Duration` (- (`self.Minutes Duration`) 10)))
  (if (== _output_get 0)
    (`self.OnTimerEnd` self))
  (return))