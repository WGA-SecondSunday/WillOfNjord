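; BP_TimeManager is an actor that runs the in-game day, hour and minute clock and manages duration-based timers.
; Tick accumulates delta time, advancing the clock in ten-minute steps and broadcasting minute, hour and day changes through dispatchers.
; CreateTimer constructs BP_Timer objects, binds their end events and hooks into minute changes, while DeleteTimer removes and unbinds them.
; Debug print handlers for hour and minute changes exist, but their bindings never run.
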(event `self.ReceiveTick`
  (params (DeltaSeconds :type "Float (single-precision)"))
  (`self.UpdateTime` DeltaSeconds))

(event `self.ReceiveBeginPlay`)

(event `OnHourChanged` :!signature `self.OnHourChange`
  (params (`New Time` :type "/Game/BP_Core/TimeManagement/BP_GameTime Structure"))
  (bind (_gametime_day _gametime_hour) (break `/Game/BP_Core/TimeManagement/BP_GameTime` (`self.GameTime`)))
  (`KismetSystemLibrary.PrintString` (`KismetStringLibrary.Concat_StrStr` "HOUR  " (`KismetStringLibrary.Conv_IntToString` _gametime_hour))))

(event `OnMinuteChanged` :!signature `self.OnMinuteChange`
  (params (`New Time` :type "/Game/BP_Core/TimeManagement/BP_GameTime Structure"))
  (bind (_gametime_day _gametime_hour _gametime_minute) (break `/Game/BP_Core/TimeManagement/BP_GameTime` (`self.GameTime`)))
  (`KismetSystemLibrary.PrintString` (`KismetStringLibrary.Concat_StrStr` (`KismetStringLibrary.Conv_IntToString` _gametime_day) " " (`KismetStringLibrary.Conv_IntToString` _gametime_hour) ":" (`KismetStringLibrary.Conv_IntToString` _gametime_minute))))

(fn `Create Timer`
  (params (Duration :type "/Game/BP_Core/TimeManagement/BP_GameTime Structure") (`On End` :type "Delegate (by ref)"))
  (bind _returnvalue (`|GenericCreateObject` "/Game/BP_Core/TimeManagement/BP_Timer.BP_Timer_C" self))
  (`KismetArrayLibrary.Array_Add` (`self.Timers`) _returnvalue)
  (`/Game/BP_Core/TimeManagement/BP_Timer.Init` _returnvalue Duration)
  (add `/Game/BP_Core/TimeManagement/BP_Timer.OnTimerEnd` _returnvalue `On End`)
  (add `/Game/BP_Core/TimeManagement/BP_Timer.OnTimerEnd` _returnvalue (`|CreateDelegate` :!event `Delete Timer`))
  (add `self.OnMinuteChange` self (`|CreateDelegate` _returnvalue :!event `Tick`))
  (return))

(fn `Delete Timer`
  (params (Timer :type "/Game/BP_Core/TimeManagement/BP_Timer Object Reference"))
  (`KismetArrayLibrary.Array_RemoveItem` (`self.Timers`) Timer)
  (remove `self.OnMinuteChange` self (`|CreateDelegate` Timer :!event `Tick`))
  (clear `/Game/BP_Core/TimeManagement/BP_Timer.OnTimerEnd` Timer)
  (return))

(fn `UpdateTime`
  (params (Delta :type "Float (double-precision)"))
  (bind (_day _hour _minute) (break `/Game/BP_Core/TimeManagement/BP_GameTime` (`self.GameTime`)))
  (bind _output_get (set `self.Elapsed` (+ Delta (`self.Elapsed`))))
  (if (>= _output_get (`self.CMinuteDuration`))
    (set `self.Elapsed` 0.0)
    (bind _output_get_2 (set `self.GameTime` (make `/Game/BP_Core/TimeManagement/BP_GameTime` _day _hour (+ _minute 10))))
    (`self.OnMinuteChange` (`self.GameTime`))
    (if (>= (`.Minute_8_834EBD4B490534C3A6916281989DF1A0` (break `/Game/BP_Core/TimeManagement/BP_GameTime` _output_get_2)) 60)
      (bind _output_get_3 (set `self.GameTime` (make `/Game/BP_Core/TimeManagement/BP_GameTime` (break `/Game/BP_Core/TimeManagement/BP_GameTime` _output_get_2) (+ (`.Hour_7_F85BF52C4A7085BDBE2839A014EE0E99` (break `/Game/BP_Core/TimeManagement/BP_GameTime` _output_get_2)) 1))))
      (`self.OnHourChange` (`self.GameTime`))
      (if (>= (`.Hour_7_F85BF52C4A7085BDBE2839A014EE0E99` (break `/Game/BP_Core/TimeManagement/BP_GameTime` _output_get_3)) 24)
        (set `self.GameTime` (make `/Game/BP_Core/TimeManagement/BP_GameTime` (+ (break `/Game/BP_Core/TimeManagement/BP_GameTime` _output_get_3) 1)))
        (`self.OnDayChange` (`self.GameTime`))
        (return)))))

(fn `UserConstructionScript`)