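; BP_Profession is a profession that holds a capped worker list and turns their labor into resource production.
; Its manager is set on Init, and AssignWorker can bypass the cap.
; MakeWork scales each producer's output by summed worker efficiency and multiplied profession and manager efficiencies, adding it to resources with a positive Goal.
; CheckConsumption tests consumer amounts against stock, but MakeWork ignores the result and deducts nothing.
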(event `Init`
  (params (Manager :type "/Game/BP_Core/ProfessionManagement/BP_ProfessionManager Object Reference"))
  (set `self.Manager` Manager))

(event `Deinit`)

(fn `AssignWorker`
  (params (Person :type "/Game/BP_Core/PeopleManagement/BP_Person Object Reference") (`Bypass Max Amount` :type Boolean))
  (returns (Added :type Boolean))
  (if (or (< (`KismetArrayLibrary.Array_Length` (`self.Workers`)) (`self.MaxWorkers`)) `Bypass Max Amount`)
    (`KismetArrayLibrary.Array_AddUnique` (`self.Workers`) Person)
    (`/Game/BP_Core/PeopleManagement/BP_Person.AssignProfession` Person self)
    (return true)
    (else
      (return false))))

(fn `CalcGlobalEfficiency`
  (returns (`Global Efficiency` :type "Float (double-precision)"))
  (locals (Eff :type "Float (double-precision)" :default 1.0))
  (for _array_element (`self.Global Efficiencies`)
    (set `local.Eff` (* (`.Efficiency_5_04ACF210425CC626F60009891486AB5D` (break `/Game/BP_Core/ProfessionManagement/BP_EfficiencyModifier` _array_element)) (`local.Eff`))))
  (return (`local.Eff`)))

(fn `CalcWorkerEfficiency`
  (returns (`People Efficiency` :type "Float (double-precision)"))
  (locals (Efficiency :type "Float (double-precision)" :default 0.0))
  (for _array_element (`self.Workers`)
    (set `local.Efficiency` (+ (`/Game/BP_Core/PeopleManagement/BP_Person.Efficiency` _array_element) (`local.Efficiency`))))
  (return (`local.Efficiency`)))

(fn `CheckConsumption`
  (params (Resources :type "/Game/BP_Core/ResourceManagement/BP_UResourceManager Object Reference (by ref)"))
  (returns (Success :type Boolean))
  (for _array_element (`self.Consumers`)
    (bind (_resource _amount) (break `/Game/BP_Core/ProfessionManagement/BP_Consumer` _array_element))
    (if (not (>= (`/Game/BP_Core/ResourceManagement/BP_UResource.Amount` (`BlueprintMapLibrary.Map_Find` (`/Game/BP_Core/ResourceManagement/BP_UResourceManager.Resources` Resources) _resource)) _amount))
      (return false)))
  (return true))

(fn `FireWorker`
  (params (Worker :type "/Game/BP_Core/PeopleManagement/BP_Person Object Reference"))
  (returns (Success :type Boolean))
  (bind _returnvalue (`KismetArrayLibrary.Array_RemoveItem` (`self.Workers`) Worker))
  (return _returnvalue))

(fn `MakeWork`
  (params (ResMan :type "/Game/BP_Core/ResourceManagement/BP_UResourceManager Object Reference (by ref)"))
  (`self.CheckConsumption` ResMan)
  (bind _global_efficiency (`self.CalcGlobalEfficiency`))
  (bind _people_efficiency (`self.CalcWorkerEfficiency`))
  (for _array_element (`self.Producers`)
    (bind (_resource _efficiency _baseproduction) (break `/Game/BP_Core/ProfessionManagement/BP_Producer` _array_element))
    (bind _value (`BlueprintMapLibrary.Map_Find` (`/Game/BP_Core/ResourceManagement/BP_UResourceManager.Resources` ResMan) _resource))
    (if (> (`/Game/BP_Core/ResourceManagement/BP_UResource.Goal` _value) 0.0)
      (`/Game/BP_Core/ResourceManagement/BP_UResource.UpdateAmount` _value (+ (* _efficiency _baseproduction _people_efficiency _global_efficiency (`/Game/BP_Core/ProfessionManagement/BP_ProfessionManager.Global Efficiency` (`self.Manager`))) (`/Game/BP_Core/ResourceManagement/BP_UResource.Amount` _value)))))
  (return))