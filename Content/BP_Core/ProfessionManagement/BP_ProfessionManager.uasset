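; Manager that owns the game's professions and triggers their work as game time passes.
; On BeginPlay it constructs and initializes one object per class in the static professions list, stores them in a class-keyed map, then binds to the time manager's hour and minute events.
; Professions flagged ProduceEvery10Minutes run MakeWork on each minute event, the rest on each hour event, each receiving the resource manager.
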(event `self.ReceiveBeginPlay`
  (bind _gtimemanager (`/Game/BP_Core/BP_Gamemode.GTimeManager` (`self.GameManager`)))
  (`parent.ReceiveBeginPlay`)
  (`self.CreateProfessions`)
  (add `/Game/BP_Core/TimeManagement/BP_TimeManager.OnHourChange` _gtimemanager (`|CreateDelegate` :!event `HandleHourTick`))
  (add `/Game/BP_Core/TimeManagement/BP_TimeManager.OnMinuteChange` _gtimemanager (`|CreateDelegate` :!event `HandleMinuteTick`)))

(fn `CreateProfessions`
  (for _array_element (`/Game/BP_Core/ProfessionManagement/BPDA_ProfMan_Data.Professions List` (`self.StaticData`))
    (bind _returnvalue (`|GenericCreateObject` _array_element self))
    (`/Game/BP_Core/ProfessionManagement/BP_Profession.Init` _returnvalue self)
    (`BlueprintMapLibrary.Map_Add` (`self.Professions`) _array_element _returnvalue))
  (return))

(fn `HandleHourTick`
  (params (`New Time` :type "/Game/BP_Core/TimeManagement/BP_GameTime Structure"))
  (`self.ProduceAll`)
  (return))

(fn `HandleMinuteTick`
  (params (Time :type "/Game/BP_Core/TimeManagement/BP_GameTime Structure"))
  (bind _values (`BlueprintMapLibrary.Map_Values` (`self.Professions`)))
  (for _array_element _values
    (if (`/Game/BP_Core/ProfessionManagement/BP_Profession.Produce Every 10 Minutes` _array_element)
      (`/Game/BP_Core/ProfessionManagement/BP_Profession.MakeWork` _array_element (`/Game/BP_Core/BP_Gamemode.GResourceManager` (`self.GameManager`))))))

(fn `ProduceAll`
  (bind _values (`BlueprintMapLibrary.Map_Values` (`self.Professions`)))
  (for _array_element _values
    (if (not (`/Game/BP_Core/ProfessionManagement/BP_Profession.Produce Every 10 Minutes` _array_element))
      (`/Game/BP_Core/ProfessionManagement/BP_Profession.MakeWork` _array_element (`/Game/BP_Core/BP_Gamemode.GResourceManager` (`self.GameManager`)))))
  (return))

(fn `UserConstructionScript`)