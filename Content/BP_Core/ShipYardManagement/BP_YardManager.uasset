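; Ship yard manager that tracks staged construction of the ship and ends the game when it is built.
; Once a yard is built, it shows the HUD progress bar and hooks the ship resource's goal-reached event.
; Goal counts fire stage events that swap the BP_Ship mesh from hidden through half-built to complete.
; Reaching the stage count flags the ship built, and Tick then pauses the game through the time manager.
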(event `self.ReceiveBeginPlay`
  (`parent.ReceiveBeginPlay`)
  (add `/Game/BP_Core/BP_Gamemode.GameInitialized` (`self.GameManager`) (delegate `CustomEvent_0`))
  (add `self.On Ship Stage Done` (delegate `On Ship Stage Done Handler`))
  (add `self.On Ship Built` (`|CreateDelegate` :!event `Ship Built Handler`))
  (bind _returnvalue (`GameplayStatics.GetActorOfClass` "/Game/BP_Core/ShipYardManagement/BP_Ship.BP_Ship_C"))
  (set `self.Ship` _returnvalue)
  (`self.Update Ship Stage` 0)
  (`KismetSystemLibrary.PrintString` "Инициализация корабельного манагера успешна"))

(event `CustomEvent_0`
  (set `self.Ship Progress Bar` (`/Game/UI/Widgets/TimerAndScreenButtons/BP_HUD.ShipProgress` (`/Game/BP_Core/BP_Gamemode.WHUD` (`self.GameManager`))))
  (`KismetSystemLibrary.PrintString` "Включен корабельный прогресс бар"))

(event `On Ship Stage Done Handler` :!signature `self.On Ship Stage Done`
  (params (`Current Stage` :type Integer))
  (`self.Update Ship Stage` `Current Stage`))

(event `self.ReceiveTick`
  (params (DeltaSeconds :type "Float (single-precision)"))
  (if (`self.Ship Built`)
    (`KismetSystemLibrary.PrintString` "GAME COMPLETED" true true (struct :`G` 0.063577 :`B` 1.0 :`A` 1.0))
    (`/Game/BP_Core/TimeManagement/BP_TimeManager.Set Game Paused` (`/Game/BP_Core/BP_Gamemode.GTimeManager` (`self.GameManager`)) true)))

(fn `Ship Built Handler`
  (set `self.Ship Built` true))

(fn `Ship Progress Tracker`
  (params (`Ship Resource` :type "/Game/BP_Core/ResourceManagement/BP_UResource Object Reference"))
  (bind _goal_reached_times (`/Game/BP_Core/ResourceManagement/BP_UResource.Goal Reached Times` `Ship Resource`))
  (if (`|EnumEquality` (`/Game/BP_Core/ResourceManagement/BP_UResource.Resource Type` `Ship Resource`) "NewEnumerator8")
    (`KismetSystemLibrary.PrintString` (`KismetTextLibrary.Conv_TextToString` (`|FormatText` "Прилетел апдейт корабля: A {amount}, G {goal}, R {reached}. Всего стадий - {stages}" (`/Game/BP_Core/ResourceManagement/BP_UResource.Amount` `Ship Resource`) (`/Game/BP_Core/ResourceManagement/BP_UResource.Goal` `Ship Resource`) (`/Game/BP_Core/ResourceManagement/BP_UResource.Goal Reached Times` `Ship Resource`) (`self.Ship Build Stages Count`))) true true (struct :`G` 0.66 :`B` 1.0 :`A` 1.0) 5.0)
    (`self.On Ship Stage Done` _goal_reached_times)
    (if (>= _goal_reached_times (`self.Ship Build Stages Count`))
      (`KismetSystemLibrary.PrintString` "Корабль построен!" true true (struct :`G` 0.66 :`B` 1.0 :`A` 1.0) 5.0)
      (`self.On Ship Built`))))

(fn `Ship Stage Done Handler`
  (params (Stage :type Integer))
  (locals (`Original Brush` :type "SlateBrush Structure"))
  (bind _middlebarimage (`/Game/UI/Widgets/TimerAndScreenButtons/BP_CustomHorizontalProgressBar.MiddleBarImage` (`self.Ship Progress Bar`)))
  (set `local.Original Brush` (`Image.Brush` _middlebarimage))
  (`Image.SetBrushTintColor` _middlebarimage (make `SlateColor` (struct :`R` 1.0 :`A` 1.0))))

(fn `Ship Yard Built Handler`
  (params (Yard :type "/Game/GameData/Buildings/ShipYard/BP_ShipYard Object Reference"))
  (bind _ship_progress_bar (`self.Ship Progress Bar`))
  (bind _value (`BlueprintMapLibrary.Map_Find` (`/Game/BP_Core/ResourceManagement/BP_UResourceManager.Resources` (`/Game/BP_Core/BP_Gamemode.GResourceManager` (`self.GameManager`))) "NewEnumerator8"))
  (`Widget.SetVisibility` _ship_progress_bar "Visible")
  (`/Game/UI/Widgets/TimerAndScreenButtons/BP_CustomHorizontalProgressBar.Init` _ship_progress_bar (`self.Ship Resource Stage Goal`) (`self.Ship Build Stages Count`) _value)
  (`/Game/BP_Core/ResourceManagement/BP_UResource.Update Goal` _value (`self.Ship Resource Stage Goal`))
  (add `/Game/BP_Core/ResourceManagement/BP_UResource.OnGoalReached` _value (`|CreateDelegate` :!event `Ship Progress Tracker`)))

(fn `Update Ship Stage`
  (params (Stage :type Integer))
  (bind _shipmesh (`/Game/BP_Core/ShipYardManagement/BP_Ship.ShipMesh` (`self.Ship`)))
  (switch `int` Stage
    (:`0`
      (`SceneComponent.SetVisibility` _shipmesh false false))
    (:`1`
      (`SceneComponent.SetVisibility` _shipmesh true false)
      (`StaticMeshComponent.SetStaticMesh` _shipmesh "/Game/Maps/MainMap/MapData/MapMaterials/DamagedShip/Ship_50_Mesh.Ship_50_Mesh"))
    (:`2`
      (`SceneComponent.SetVisibility` _shipmesh true false)
      (`StaticMeshComponent.SetStaticMesh` _shipmesh "/Game/Maps/MainMap/MapData/MapMaterials/DamagedShip/Ship_Mesh.Ship_Mesh"))))

(fn `UserConstructionScript`
  (`parent.UserConstructionScript`))