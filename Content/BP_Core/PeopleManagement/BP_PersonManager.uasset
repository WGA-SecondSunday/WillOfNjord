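; BP_PersonManager creates and holds the game's population of BP_Person objects and provides their AI bodies.
; Once the gamemode signals initialization, it tops the People list up to the initial count, optionally randomizing each person's efficiency, and broadcasts OnPeopleAdded per person.
; AddAIMesh spawns an AI character running the BPBT_NoProf behavior tree at a random navigable point around BP_InitialTargetPoint and links it to the person.
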(event `self.ReceiveBeginPlay`
  (`parent.ReceiveBeginPlay`)
  (add `/Game/BP_Core/BP_Gamemode.GameInitialized` (cast `/Game/BP_Core/BP_Gamemode` (`GameplayStatics.GetGameMode`) :!pure true) (delegate `CustomEvent_0`)))

(event `CustomEvent_0`
  (`self.Add People` (`self.InitialPeopleCount`) true))

(fn `Add AI Mesh`
  (params (Person :type "/Game/BP_Core/PeopleManagement/BP_Person Object Reference"))
  (bind _returnvalue (`GameplayStatics.GetActorOfClass` "/Game/AI_Pawn/TargetPoints/BP_InitialTargetPoint.BP_InitialTargetPoint_C"))
  (bind _returnvalue_2 (`AIBlueprintHelperLibrary.SpawnAIFromClass` "/Game/AI_Pawn/MyAICharacter_2.MyAICharacter_2_C" "/Game/AI_Pawn/Professions/NoProfession/BPBT_NoProf.BPBT_NoProf" (`NavigationSystemV1.K2_GetRandomLocationInNavigableRadius` (`self.K2_GetActorLocation` _returnvalue) 2000.0 null null) (`KismetMathLibrary.MakeRotator` 0.0 0.0 (`KismetMathLibrary.Conv_IntToDouble` (`KismetMathLibrary.RandomIntegerInRange` 0 360))) true null))
  (bind _asmy_aicharacter_2 (cast `/Game/AI_Pawn/MyAICharacter_2` _returnvalue_2))
  (set `/Game/BP_Core/PeopleManagement/BP_Person.Linked AI` _asmy_aicharacter_2 Person))

(fn `Add People`
  (params (Count :type Integer) (`Random Efficiencies` :type Boolean))
  (locals (PeopleCount :type Integer))
  (while (< (`local.PeopleCount`) Count)
    (`/Engine/EditorBlueprintResources/StandardMacros.IncrementInt` (`local.PeopleCount`)
      (:`  `
        (bind _returnvalue (`|GenericCreateObject` "/Game/BP_Core/PeopleManagement/BP_Person.BP_Person_C" self))
        (if `Random Efficiencies`
          (set `/Game/BP_Core/PeopleManagement/BP_Person.Efficiency` (`KismetMathLibrary.RandomFloatInRange` 0.0 1.0) _returnvalue))
        (`KismetArrayLibrary.Array_Add` (`self.People`) _returnvalue)
        (`self.OnPeopleAdded` _returnvalue))))
  (return))

(fn `UserConstructionScript`
  (locals (End :type Integer :default 5) (Curr :type Integer))
  (add `self.OnPeopleAdded` (`|CreateDelegate` :!event `Add AI Mesh`)))