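; Top-down camera pawn for the main map, with clamped panning at a fixed height and mouse-wheel spring-arm zoom.
; Holding right-click hides the cursor and enables rotation within the camera manager's pitch and yaw limits set at BeginPlay.
; A delayed key check separates clicks from holds.
; Clicks trace under the cursor and glide the pawn to the hit actor via a timeline lerp, ignoring the Landscape by display name.
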(event `self.ReceiveBeginPlay`
  (bind _returnvalue (`GameplayStatics.GetPlayerCameraManager` 0))
  (`Controller.SetControlRotation` (`GameplayStatics.GetPlayerController` 0) (`KismetMathLibrary.MakeRotator` 0.0 300.0))
  (`self.K2_SetActorLocation` (-20000.0 3000.0 7000.0))
  (set `PlayerCameraManager.ViewYawMax` 80.0 _returnvalue)
  (set `PlayerCameraManager.ViewYawMin` -80.0 _returnvalue)
  (set `PlayerCameraManager.ViewPitchMin` 300.0 _returnvalue)
  (set `PlayerCameraManager.ViewPitchMax` 345.0 _returnvalue)
  (set `SpringArmComponent.TargetArmLength` 10000.0 (`self.SpringArm`)))

(event `InputAction|RightClick`
  (params (Key :type "Key Structure"))
  (bind _returnvalue (`GameplayStatics.GetPlayerController` 0))
  (:`Pressed`
    (`KismetSystemLibrary.Delay` 0.02)
    (set `self.Right_Click_Held` true)
    (bind _asbp_our_player_controller (cast `/Game/Maps/MainMap/BP_OurPlayerController` _returnvalue))
    (set `/Game/Maps/MainMap/BP_OurPlayerController.RightClickHeld` true _asbp_our_player_controller)
    (set `PlayerController.bShowMouseCursor` false _asbp_our_player_controller))
  (:`Released`
    (set `self.Right_Click_Held` false)
    (bind _asbp_our_player_controller_2 (cast `/Game/Maps/MainMap/BP_OurPlayerController` _returnvalue))
    (set `/Game/Maps/MainMap/BP_OurPlayerController.RightClickHeld` false _asbp_our_player_controller_2)
    (set `PlayerController.bShowMouseCursor` true _asbp_our_player_controller_2)
    (`WidgetBlueprintLibrary.SetInputMode_GameAndUIEx` _asbp_our_player_controller_2 null "DoNotLock" false)))

(event `InputAction|Click`
  (params (Key :type "Key Structure"))
  (:`Pressed`
    (`KismetSystemLibrary.Delay` 0.2)
    (`self.HandleMouseClick` Key))
  (:`Released`
    (set `self.Click_Held` false)))

(event `MoveToFocusActor`
  (params (Focused_Actor :type "Actor Object Reference"))
  (bind (_direction _animationcurve) (`Timeline|FocusedTimeline` :!via `PlayFromStart`)
    (:`Update`
      (`self.K2_SetActorLocation` (`KismetMathLibrary.VLerp` (`self.K2_GetActorLocation`) (`self.K2_GetActorLocation` Focused_Actor) _animationcurve)))))

(event `Key|MouseScrollUp`
  (params (Key :type "Key Structure"))
  (bind _springarm (`self.SpringArm`))
  (bind _targetarmlength (`SpringArmComponent.TargetArmLength` _springarm))
  (:`Pressed`
    (if (>= _targetarmlength 2000.0)
      (set `SpringArmComponent.TargetArmLength` (+ _targetarmlength -500.0) _springarm))))

(event `Key|MouseScrollDown`
  (params (Key :type "Key Structure"))
  (bind _springarm (`self.SpringArm`))
  (bind _targetarmlength (`SpringArmComponent.TargetArmLength` _springarm))
  (:`Pressed`
    (if (<= _targetarmlength 15000.0)
      (set `SpringArmComponent.TargetArmLength` (+ _targetarmlength 600.0) _springarm))))

(event `InputAxisKey|MouseX`
  (params (AxisValue :type "Float (single-precision)"))
  (if (`self.Right_Click_Held`)
    (`self.AddControllerYawInput` AxisValue)))

(event `InputAxisKey|MouseY`
  (params (AxisValue :type "Float (single-precision)"))
  (if (`self.Right_Click_Held`)
    (`self.AddControllerPitchInput` (* AxisValue -1.0))))

(event `InputAxis|PlayerMoveForward`
  (params (AxisValue :type "Float (single-precision)"))
  (`self.K2_SetActorLocation` (`KismetMathLibrary.MakeVector` (`KismetMathLibrary.FClamp` (.x (+ (`self.K2_GetActorLocation`) (* (`self.GetActorForwardVector` (`GameplayStatics.GetPlayerCameraManager` 0)) AxisValue))) -30000.0 20000.0) (`KismetMathLibrary.FClamp` (.y (+ (`self.K2_GetActorLocation`) (* (`self.GetActorForwardVector` (`GameplayStatics.GetPlayerCameraManager` 0)) AxisValue))) -25000.0 25000.0) (`KismetMathLibrary.FClamp` (.z (+ (`self.K2_GetActorLocation`) (* (`self.GetActorForwardVector` (`GameplayStatics.GetPlayerCameraManager` 0)) AxisValue))) 7000.0 7000.0))))

(event `InputAxis|PlayerMoveRight`
  (params (AxisValue :type "Float (single-precision)"))
  (`self.K2_SetActorLocation` (`KismetMathLibrary.MakeVector` (`KismetMathLibrary.FClamp` (.x (+ (`self.K2_GetActorLocation`) (* (`self.GetActorRightVector` (`GameplayStatics.GetPlayerCameraManager` 0)) AxisValue))) -30000.0 20000.0) (`KismetMathLibrary.FClamp` (.y (+ (`self.K2_GetActorLocation`) (* (`self.GetActorRightVector` (`GameplayStatics.GetPlayerCameraManager` 0)) AxisValue))) -25000.0 25000.0) (`KismetMathLibrary.FClamp` (.z (+ (`self.K2_GetActorLocation`) (* (`self.GetActorRightVector` (`GameplayStatics.GetPlayerCameraManager` 0)) AxisValue))) 7000.0 7000.0))))

(fn `Change_Arm_Length`
  (bind _springarm (`self.SpringArm`))
  (set `SpringArmComponent.TargetArmLength` (+ (`SpringArmComponent.TargetArmLength` _springarm) (`self.Delta_TargetArm`)) _springarm))

(fn `CheckIfCLickHitActor`
  (returns (bBlockingHit :type Boolean) (HitActor :type "Actor Object Reference"))
  (bind (_bblockinghit _binitialoverlap _time _distance _location _impactpoint _normal _impactnormal _physmat _hitactor) (`GameplayStatics.BreakHitResult` (`PlayerController.GetHitResultUnderCursorByChannel` (`GameplayStatics.GetPlayerController` 0) "TraceTypeQuery1" true)))
  (return _bblockinghit _hitactor))

(fn `HandleMouseClick`
  (params (Key :type "Key Structure" :default "None"))
  (bind (_bblockinghit _hitactor) (`self.CheckIfCLickHitActor`))
  (bind _returnvalue (`PlayerController.IsInputKeyDown` (`GameplayStatics.GetPlayerController` 0) Key))
  (if _returnvalue
    (set `self.Click_Held` _returnvalue)
    (elif _bblockinghit
      (bind _output_get (set `self.Focused_Actor` _hitactor))
      (bind _returnvalue_2 (`KismetSystemLibrary.GetDisplayName` _output_get))
      (if (`KismetStringLibrary.NotEqual_StrStr` _returnvalue_2 "Landscape")
        (`self.MoveToFocusActor` _output_get)
        (`KismetSystemLibrary.PrintString` _returnvalue_2)))))

(fn `PrintWorldLocation`
  (`KismetSystemLibrary.PrintString` "scene")
  (`KismetSystemLibrary.PrintString` (`KismetStringLibrary.Conv_VectorToString` (`SceneComponent.K2_GetComponentLocation` (`self.Scene`))))
  (`KismetSystemLibrary.PrintString` "Arm")
  (`KismetSystemLibrary.PrintString` (`KismetStringLibrary.Conv_VectorToString` (`SceneComponent.K2_GetComponentLocation` (`self.SpringArm`))))
  (`KismetSystemLibrary.PrintString` "Camera")
  (`KismetSystemLibrary.PrintString` (`KismetStringLibrary.Conv_VectorToString` (`SceneComponent.K2_GetComponentLocation` (`self.Camera`))))
  (`KismetSystemLibrary.PrintString` (`KismetStringLibrary.Conv_RotatorToString` (`SceneComponent.K2_GetComponentRotation` (`self.Scene`))))
  (`KismetSystemLibrary.PrintString` (`KismetStringLibrary.Conv_RotatorToString` (`SceneComponent.K2_GetComponentRotation` (`self.SpringArm`))))
  (`KismetSystemLibrary.PrintString` (`KismetStringLibrary.Conv_RotatorToString` (`SceneComponent.K2_GetComponentRotation` (`self.Camera`)))))

(fn `UserConstructionScript`
  (set `self.Target Arm Length` (`SpringArmComponent.TargetArmLength` (`self.SpringArm`))))